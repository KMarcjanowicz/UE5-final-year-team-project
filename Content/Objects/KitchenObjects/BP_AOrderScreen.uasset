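; BP_AOrderScreen is a kitchen screen that shows the name of a single recipe order.
; DisplayOrder takes a recipe, stores its ID and name, flags the screen as occupied through HasOrder and writes the name to OrderText.
; CleanScreen clears the flag and resets the text to a placeholder, while the construction script starts the screen with no order.
; The event graph holds no active logic.
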(event EventBeginPlay)

(event Collision|EventActorBeginOverlap
  (params (OtherActor :type Actor%20Object%20Reference)))

(event EventTick
  (params (DeltaSeconds :type Float%20%28single-precision%29)))

(fn ConstructionScript
  (Variables|Default|SetbHasOrder false))

(fn DisplayOrder
  (params (_Recipe :type S%20Recipe%20Structure))
  (bind (_id _ingredientsid _toolsid _name) (Utilities|Struct|BreakSRecipe _Recipe))
  (Variables|Default|SetOrderID _id)
  (Variables|Default|SetbHasOrder true)
  (bind _output_get (Variables|Default|SetOrderName _name))
  (Rendering|Components|TextRender|SetText (Variables|Default|GetOrderText) (Utilities|Text|ToText(Name) _output_get)))

(fn CleanScreen
  (Variables|Default|SetbHasOrder false)
  (Rendering|Components|TextRender|SetText (Variables|Default|GetOrderText) (Utilities|Text|ToText(String) "...")))