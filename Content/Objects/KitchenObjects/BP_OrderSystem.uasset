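; Kitchen order manager that generates random stew, borgor or pizzer orders and shows them on the level's BP_OrderScreen actors.
; A one-second looping timer adds an order after a time threshold or by random chance, until a counter, never decremented here, hits its maximum.
; Recipes from DT_Recipes fill parallel arrays tracking processed and sent state, feeding free screens.
; SendOrder matches screen and order IDs, clears the screen, flags processed orders sent and refreshes displays.
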(event EventBeginPlay
  (Utilities|Time|SetTimerbyFunctionName 0 "OrderComeIn" 1.0 true))

(event Collision|EventActorBeginOverlap
  (params (OtherActor :type Actor%20Object%20Reference)))

(event EventTick
  (params (DeltaSeconds :type Float%20%28single-precision%29)))

(fn ConstructionScript
  (Variables|Default|SetMaxNumberOfOrders 3.0)
  (Variables|Default|SetChanceOfReceivingOrder 0.2)
  (Variables|Default|SetTimeOffsetForOrders 3e+01)
  (Variables|Default|SetNumberOfOrders 0.0)
  (bind _outactors (Actor|GetAllActorsOfClass "/Game/Objects/KitchenObjects/BP_OrderScreen.BP_OrderScreen_C"))
  (Variables|Default|SetOrderScreens _outactors))

(fn OrderComein
  ;[1 1 1] Printing seconds since last order
  (Variables|Default|SetSecondsPassedSinceLastOrder (+ (Variables|Default|GetSecondsPassedSinceLastOrder) 1.0))
  (if (not (>= (Variables|Default|GetNumberOfOrders) (Variables|Default|GetMaxNumberOfOrders))) ; if we didn't hit the max number of orders
    (if (>= (Variables|Default|GetSecondsPassedSinceLastOrder) (Variables|Default|GetTimeOffsetForOrders)) ; if it doesn't hit the time treshhold
      (CallFunction|FetchOrder :!label _label) ; Random order and call to add to the order displays
      (Variables|Default|SetSecondsPassedSinceLastOrder 0.0)
      (Variables|Default|SetNumberOfOrders (+ (Variables|Default|GetNumberOfOrders) 1.0))
      (elif (<= (Math|Random|RandomFloatinRange 0.0 1.0) (* (Variables|Default|GetChanceOfReceivingOrder) 1.15)) ; Random chance of getting the order early
        (goto _label)))))

(fn AddOrdertoDisplayScreen
  (for _array_element (Variables|Default|GetOrderScreens)
    (if (not (Variables|/Game/Objects/KitchenObjects/BP_OrderScreen.BP_OrderScreen_C|GetbHasOrder _array_element))
      (for _index (range 0 (- (Utilities|Array|Length (Variables|Default|GetOrderRecipes)) 1))
        (if (Class|KismetMathLibrary|XORBoolean (Math|Boolean|NORBoolean (Variables|/Game/Objects/KitchenObjects/BP_OrderScreen.BP_OrderScreen_C|GetbHasOrder _array_element) (Utilities|Array|Get(acopy) (Variables|Default|GetOrderProcessed) _index)) (Utilities|Array|Get(acopy) (Variables|Default|GetOrderSent) _index))
          (Utilities|Array|SetArrayElem (Variables|Default|GetOrderProcessed) _index true)
          (Default|DisplayOrder _array_element (Utilities|Array|Get(acopy) (Variables|Default|GetOrderRecipes) _index))))
      (else
        (Development|PrintString "Screen already has order displayed")))))

(fn FetchOrder
  (LocalVariables|Set_RecipeNumber (Math|Random|RandomIntegerinRange 1 3))
  (if (== (LocalVariables|Get_RecipeNumber) 1)
    (bind _returnvalue (Utilities|GetDataTableRow "/Game/Objects/DT_Recipes.DT_Recipes" "StewRecipe")
      (:then
        (Utilities|Array|Add (Variables|Default|GetOrderRecipes) _returnvalue)
        (Utilities|Array|Add (Variables|Default|GetOrderProcessed) false :!label _label)
        (Utilities|Array|Add (Variables|Default|GetOrderSent) false)
        (CallFunction|AddOrdertoDisplayScreen)))
    (elif (== (LocalVariables|Get_RecipeNumber) 2)
      (bind _returnvalue_2 (Utilities|GetDataTableRow "/Game/Objects/DT_Recipes.DT_Recipes" "BorgorRecipe")
        (:then
          (Utilities|Array|Add (Variables|Default|GetOrderRecipes) _returnvalue_2)
          (goto _label)))
      (elif (== (LocalVariables|Get_RecipeNumber) 3)
        (bind _returnvalue_3 (Utilities|GetDataTableRow "/Game/Objects/DT_Recipes.DT_Recipes" "PizzerRecipe")
          (:then
            (Utilities|Array|Add (Variables|Default|GetOrderRecipes) _returnvalue_3)
            (goto _label)))))))

(fn SendOrder
  (params (_OrderID :type Integer) (_ScreenID :type Integer))
  ;[1 1 1] Check is recipe matches the order and then if screen matches the serving area
  (for _array_element (Variables|Default|GetOrderScreens)
    (if (== (Variables|/Game/Objects/KitchenObjects/BP_OrderScreen.BP_OrderScreen_C|GetScreenID _array_element) _ScreenID)
      (if (== (Variables|/Game/Objects/KitchenObjects/BP_OrderScreen.BP_OrderScreen_C|GetOrderID _array_element) _OrderID)
        ;[1 1 1] Checkif the order wasn't already sent & check if it was processed. Mark as send if true.
        (Default|CleanScreen _array_element)
        (for _index (range 0 (- (Utilities|Array|Length (Variables|Default|GetOrderProcessed)) 1))
          (if (and (Utilities|Array|Get(acopy) (Variables|Default|GetOrderProcessed) _index) (== (Variables|/Game/Objects/KitchenObjects/BP_OrderScreen.BP_OrderScreen_C|GetOrderID _array_element) _OrderID))
            (Utilities|Array|SetArrayElem (Variables|Default|GetOrderSent) _index true)
            (CallFunction|AddOrdertoDisplayScreen)))
        (else
          (Development|PrintString "false order id")))
      (else
        (Development|PrintString "Order doesn't match with the screen order")))))