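; BP_AShutter is an unfinished kitchen shutter actor meant to open and close.
; The construction script sets IsOpen to true, and clicking the actor prints a debug message and calls OpenShutter.
; OpenShutter only checks whether the shutter is closed and then does nothing, and CloseShutter is empty.
; The click event is noted as not working, and BeginPlay, overlap and Tick are disabled.
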(event EventBeginPlay
  (|CallParentFunction) ; This node is disabled and will not be called.\nDrag off pins to build functionality.
)

(event Collision|EventActorBeginOverlap
  (params (OtherActor :type Actor%20Object%20Reference))
  (|CallParentFunction OtherActor) ; This node is disabled and will not be called.\nDrag off pins to build functionality.
)

(event EventTick
  (params (DeltaSeconds :type Float%20%28single-precision%29))
  (|CallParentFunction DeltaSeconds) ; This node is disabled and will not be called.\nDrag off pins to build functionality.
)

(event MouseInput|EventActorOnClicked
  (params (ButtonPressed :type Key%20Structure :default "None"))
  (Development|PrintString "Actor has been clicked")
  (CallFunction|OpenShutter))

(fn ConstructionScript
  (|CallParentFunction)
  (Variables|Default|SetbIsOpen true))

(fn OpenShutter
  (if (not (Variables|Default|GetbIsOpen)) ; check if it is not open
    _))

(fn CloseShutter)