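; Serving area actor where the player plates a finished meal to submit it as an order.
; Plate rejects non-meals and ignores calls while busy, then looks up the item in DT_Objects and spawns its Blueprint on the mesh's first socket.
; It frees the active tentacle's inventory slot and sends order ID, screen ID and reward score to BP_OrderSystem.
; After a short pickup delay it destroys the meal and becomes available again.
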(event EventPlate
  (params (_item :type S%20Inventory%20Item%20Structure%20%28by%20ref%29))
  (bind (_id _displayname _type _holdingtentacleid _databasereferencename) (Utilities|Struct|BreakS_InventoryItem _item))
  (if (not (Variables|Default|GetbIsBusy))
    (if (Utilities|Enum|Equal(Enum) _type "NewEnumerator2")
      (bind __objectitem (CallFunction|FetchfromDataTable _databasereferencename))
      (CallFunction|AttachActor __objectitem)
      (CallFunction|RemoveItem)
      (bind (__score __orderid) (CallFunction|GetScore __objectitem))
      (Default|SendOrder (Variables|Default|GetOrderSystem) __orderid (Variables|Default|GetID) __score)
      (Utilities|FlowControl|Delay 3.0) ; this is when alien silhuette comes in to pick up order
      (CallFunction|DetachActor)
      (else
        (Development|PrintString "Is not meal!" true true "(R=1.000000,G=0.000000,B=0.027591,A=1.000000)")))))

(fn ConstructionScript
  (|CallParentFunction)
  (bind _returnvalue (Actor|GetActorOfClass "/Game/Blueprints/KitchenObjects/BP_OrderSystem.BP_OrderSystem_C"))
  (Variables|Default|SetOrderSystem _returnvalue))

(fn FetchfromDataTable
  (params (_DataTableRef :type Name))
  (bind _returnvalue (Utilities|GetDataTableRow "/Game/Blueprints/DT_Objects.DT_Objects" _DataTableRef)
    (:then
      (Development|PrintString (Utilities|String|Append (Utilities|String|Append "Found item " (.DisplayName (Utilities|Struct|BreakS_Object _returnvalue))) "in the data base"))
      (return _returnvalue))))

(fn AttachActor
  (params (_Item :type S%20Object%20Structure))
  (CallFunction|SetUpMealActor (.Placeholderforblueprint (Utilities|Struct|BreakS_Object _Item))))

(fn SetUpMealActor
  (params (_FoodActor :type BP%20A%20Interactable%20Item%20Class%20Reference))
  (bind _staticmesh (Variables|Default|GetStaticMesh))
  (bind _staticmesh_2 (Variables|Default|GetStaticMesh))
  (bind _returnvalue (Game|SpawnActorfromClass _FoodActor (Transformation|GetSocketTransform _staticmesh_2 (Utilities|Array|Get(acopy) (Transformation|GetAllSocketNames _staticmesh_2)) "RTS_World") "AlwaysSpawn" 0 0)) ; Crockery First
  (bind _output_get (LocalVariables|Set_Food _returnvalue))
  (Physics|SetSimulatePhysics (Variables|/Game/Blueprints/BP_AInteractableItem.BP_AInteractableItem_C|GetStaticMesh _output_get) false)
  (Class|BPIPickUp|SetinUse(Message) _output_get true)
  (Transformation|AttachComponentToComponent _output_get _staticmesh (Utilities|Array|Get(acopy) (Transformation|GetAllSocketNames _staticmesh)) "KeepWorld" "KeepWorld" "KeepWorld" true)
  ;[1 1 1] for deletion later down the line
  (Utilities|Array|Add (Variables|Default|GetMealActorRef) (LocalVariables|Get_Food))
  (Variables|Default|SetbIsBusy true))

(fn DetachActor
  (for _array_element (Variables|Default|GetMealActorRef)
    (Actor|DestroyActor _array_element))
  (Variables|Default|SetbIsBusy false))

(fn RemoveItem
  (bind __activetentacle (Class|BPIPlayerController|ActiveTentacle(Message) (Game|GetPlayerController 0)))
  (bind _asbp_first_person_character (Utilities|Casting|CastToBP_FirstPersonCharacter (Game|Player|GetPlayerPawn 0)))
  (Default|RemoveItem (Variables|/Game/Blueprints/Actor/BP_FirstPersonCharacter.BP_FirstPersonCharacter_C|GetBP_AC_Inventory _asbp_first_person_character) __activetentacle)
  (Default|SetTentacleFree _asbp_first_person_character __activetentacle))

(fn GetScore
  (params (_Object :type S%20Object%20Structure))
  (bind (_id _ingredientsid _toolsid _name _displayname _timetocook _timestart _timeend _placeholderforblueprint _rewardvalue) (Utilities|Struct|BreakS_Object _Object))
  (Development|PrintString (Utilities|String|ToString(Integer) _id))
  (return _rewardvalue _id))