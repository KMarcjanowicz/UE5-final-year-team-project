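; Cutting board appliance Blueprint, prefixed OLD, that snaps overlapping ingredient items onto sockets on its static mesh.
; On actor overlap it casts to BP_AInteractableItem, checks the ingredient type, then attaches the item to the first free of three sockets.
; Per-socket empty flags start true in the construction script and are only cleared here.
; The first and third branches check different socket indices from the ones they attach to.
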(event EventBeginPlay
  (|CallParentFunction) ; This node is disabled and will not be called.\nDrag off pins to build functionality.
)

(event Collision|EventActorBeginOverlap
  (params (OtherActor :type Actor%20Object%20Reference))
  (bind _self self)
  (bind _self_2 self)
  (bind _staticmesh (Variables|Default|GetStaticMesh _self))
  (bind _returnvalue (Transformation|GetAllSocketNames _staticmesh))
  (bind _output (Utilities|Array|Get(acopy) _returnvalue 2))
  (bind _output_2 (Utilities|Array|Get(acopy) _returnvalue))
  (bind _output_3 (Utilities|Array|Get(acopy) _returnvalue 1))
  ;[1 1 1] Attach to socket
  (Variables|Default|SetOther%20Actor OtherActor)
  (|CallParentFunction OtherActor)
  (bind _asbp_ainteractable_item (Utilities|Casting|CastToBP_AInteractableItem OtherActor)
    (:then
      (if true
        (if (Utilities|Enum|Equal(Enum) (Variables|/Game/Blueprints/BP_AInteractableItem.BP_AInteractableItem_C|GetType _asbp_ainteractable_item) "NewEnumerator1")
          (if (and (Transformation|DoesSocketExist (Variables|Default|GetStaticMesh) _output) (Variables|Default|GetbSocket0Empty))
            (Transformation|AttachActorToActor (Variables|Default|GetOther%20Actor) _self_2 _output_2 "KeepRelative" "KeepRelative" "KeepRelative" true)
            (Variables|Default|SetbSocket0Empty false)
            (elif (and (Transformation|DoesSocketExist (Variables|Default|GetStaticMesh) _output_3) (Variables|Default|GetbSocket1Empty))
              (Transformation|AttachActorToActor (Variables|Default|GetOther%20Actor) _self_2 _output_3 "KeepRelative" "KeepRelative" "KeepRelative" true)
              (Variables|Default|SetbSocket1Empty false)
              (elif (and (Transformation|DoesSocketExist (Variables|Default|GetStaticMesh) _output_2) (Variables|Default|GetbSocket2Empty))
                (Transformation|AttachActorToActor (Variables|Default|GetOther%20Actor) _self_2 _output "KeepRelative" "KeepRelative" "KeepRelative" true)
                (Variables|Default|SetbSocket2Empty false)
                (else
                  (Development|PrintString "no free sockets")))))
          (else
            (Development|PrintString "Item is not an ingridient")))
        (else
          (Development|PrintString "\"Cast failed, class is not interactable object\"" :!label _label))))
    (:CastFailed
      (goto _label))))

(event EventTick
  (params (DeltaSeconds :type Float%20%28single-precision%29))
  (|CallParentFunction DeltaSeconds) ; This node is disabled and will not be called.\nDrag off pins to build functionality.
)

(fn ConstructionScript
  (|CallParentFunction)
  (Variables|Default|SetbSocket0Empty true)
  (Variables|Default|SetbSocket1Empty true)
  (Variables|Default|SetbSocket2Empty true))