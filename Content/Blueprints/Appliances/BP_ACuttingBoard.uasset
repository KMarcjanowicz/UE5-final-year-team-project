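; Cutting board appliance that holds one ingredient and turns it into its processed version for the player's tentacle-based kitchen interactions.
; Added items are looked up in the database, spawned and attached to FoodSocket without physics.
; Turning on marks the active tentacle busy with a placeholder inventory item, then spawns the processed version on the socket.
; Retrieve returns ProcessedItem as an inventory item; older tool-and-recipe matching logic is disconnected.
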(event EventOn
  (if (> (Utilities|Array|Length (Variables|Default|GetIngredientIDs)) 0)
    (CallFunction|Turnon)))

(fn ConstructionScript
  (|CallParentFunction)
  (Variables|Default|SetbIsActiveAppliance true)
  (Variables|Default|SetType "NewEnumerator4")
  (Variables|Default|SetIngredientCap 1)
  (Variables|Default|SetName "Cutting Board"))

(fn Retrieve
  (params (_ActiveTentacleID :type Integer))
  (bind _processed_item (Variables|Default|GetProcessed%20Item))
  (bind (_id _ingredientsid _toolsid _name _displayname _timetocook _timestart _timeend _placeholderforblueprint _rewardvalue _itemtype) (Utilities|Struct|BreakS_Object _processed_item))
  (return (Utilities|Struct|MakeS_InventoryItem _id _displayname _itemtype _ActiveTentacleID _name)))

(fn Turnon
  (bind _attacheditem (Variables|Default|GetAttachedItem))
  (bind (_id _ingredientsid _toolsid _name _displayname _timetocook _timestart _timeend _placeholderforblueprint _rewardvalue _itemtype _processed) (Utilities|Struct|BreakS_Object _attacheditem))
  (|CallParentFunction)
  ;[0.2993 0.8699 1] Set tentacle using this appliance as busy
  (bind __activetentacle (Class|BPIPlayerController|ActiveTentacle(Message) (Game|GetPlayerController 0)))
  (bind _asbp_first_person_character (Utilities|Casting|CastToBP_FirstPersonCharacter (Game|Player|GetPlayerPawn 0)))
  (Default|SetTentacleBusy _asbp_first_person_character __activetentacle)
  (Development|PrintString (Utilities|String|Append (Utilities|String|ToString(Integer) __activetentacle) " was set to busy"))
  (Default|AddItem (Variables|/Game/Blueprints/Actor/BP_FirstPersonCharacter.BP_FirstPersonCharacter_C|GetBP_AC_Inventory _asbp_first_person_character) "x" __activetentacle -1 "NewEnumerator7" "N/A") ; temp item to show that tentacle busy
  (if (!= _id 0)
    (bind __item (CallFunction|FetchfromDatabase _processed))
    (CallFunction|AttachItem __item)))

(fn AttachItem
  (params (_Item :type S%20Object%20Structure))
  ;[1 1 1] this needs to go when sent item to the cutting board
  (bind _returnvalue (Game|SpawnActorfromClass (.Placeholderforblueprint (Utilities|Struct|BreakS_Object _Item)) (Math|Transform|MakeTransform (Transformation|GetSocketLocation (Variables|Default|GetStaticMesh) "FoodSocket")) "AlwaysSpawn" self 0))
  (Transformation|AttachActorToActor _returnvalue self "FoodSocket" "KeepRelative" "KeepRelative" "KeepRelative" true)
  (Physics|SetSimulatePhysics (Variables|/Game/Blueprints/BP_AInteractableItem.BP_AInteractableItem_C|GetStaticMesh _returnvalue) false))

(fn AddItem
  (params (_Item :type S%20Inventory%20Item%20Structure))
  (|CallParentFunction _Item)
  (bind __item (CallFunction|FetchfromDatabase (.DatabaseReferenceName (Utilities|Struct|BreakS_InventoryItem _Item))))
  (CallFunction|AttachItem __item)
  (Variables|Default|SetAttachedItem __item))