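; Older pot appliance (by its name) that cooks added ingredients into a recipe result, or into incorrect or burnt food.
; BeginPlay caches recipe rows from DT_Objects; TurnOn matches ingredient IDs regardless of order, sets ProcessedItem and starts boiling sound.
; An empty TimerFunc serves as a stopwatch that Tick polls to switch cooking, finished and burnt smoke; Retrieve returns the result as an inventory item.
; A legacy click handler with actor spawning remains.
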(event EventTick
  (params (DeltaSeconds :type Float%20%28single-precision%29))
  (bind _returnvalue (Class|KismetSystemLibrary|GetTimerElapsedTime 0 "TimerFunc"))
  ;[1 1 1] Play relavent some animation based on how cooked the meal is
  (if (Variables|Default|GetbIsOn)
    (if (> _returnvalue (* (Variables|Default|GetCookingTime) 1.5)) ; If food is burnt, play burnt smoke
      ;;[1 1 1] THIS NEEDS NEW SMOKE EFFECT
      (Components|Activation|Activate (Variables|Default|GetSmokeFinish) false)
      (Components|Activation|Deactivate (Variables|Default|GetSmokeConstant))
      (Components|Activation|Activate (Variables|Default|GetSmokeBurned) false)
      ;[0.1823 0.07252 0] food burnt
      (bind __item (CallFunction|FetchfromDatabase "BurntRecipe"))
      (Variables|Default|SetProcessed%20Item __item)
      (Variables|Default|SetbHoldsProcessedItem true :!label _label)
      (Utilities|Array|Clear (Variables|Default|GetIngredientIDs))
      (elif (and (> _returnvalue (Variables|Default|GetCookingTime)) (not (Variables|Default|GetbHoldsProcessedItem))) ; If food is cooked play big smoke
        (Components|Activation|Activate (Variables|Default|GetSmokeFinish) false)
        (goto _label)
        (else
          (Components|Activation|Activate (Variables|Default|GetSmokeConstant) false) ; If food is cooking but not yet done play small smoke
        )))))

(event EventBeginPlay
  ;[1 1 1] Get the recipes from the data table
  (bind _outrownames (DataTable|GetDataTableRowNames "/Game/Blueprints/DT_Objects.DT_Objects"))
  (for _array_element _outrownames
    (bind _returnvalue (Utilities|GetDataTableRow "/Game/Blueprints/DT_Objects.DT_Objects" _array_element)
      (:then
        (if (Utilities|Enum|Equal(Enum) (.ItemType (Utilities|Struct|BreakS_Object _returnvalue)) "NewEnumerator2")
          (Utilities|Array|Add (Variables|Default|GetRecipes) _returnvalue))))))

(fn ConstructionScript
  (|CallParentFunction)
  (Variables|Default|SetbIsActiveAppliance false)
  (Variables|Default|SetIngredientCap 5)
  (Variables|Default|SetType "NewEnumerator4")
  (Variables|Default|SetName "Pot"))

(fn ClickedOn-Old
  (params (GrabbedObject :type Actor%20Object%20Reference) (ObjectTypeGrabbed :type E_ItemTypes%20Enum :default "NewEnumerator0"))
  (bind _returnvalue (Class|KismetSystemLibrary|GetTimerElapsedTime 0 "FUNC"))
  (bind _returnvalue_2 (Transformation|GetActorLocation))
  (bind _cookingtime (Variables|Default|GetCookingTime))
  (bind _returnvalue_3 (+ _returnvalue_2 "0,0.000000,100.000000"))
  (bind _returnvalue_4 (Math|Conversions|ToTransform(Vector) _returnvalue_3))
  (if (Utilities|Enum|Equal(Enum) ObjectTypeGrabbed "NewEnumerator1") ; If Holding ingredient add it to the appliance, else turn it on/get recipe out
    (bind _asbp_aingredient (Utilities|Casting|CastToBP_AIngredient GrabbedObject))
    (Utilities|Array|AddUnique (Variables|Default|GetIngredientIDs) (Variables|/Game/Blueprints/BP_AInteractableItem.BP_AInteractableItem_C|GetID _asbp_aingredient))
    (Development|PrintString "Added")
    (elif (Variables|Default|GetbIsOn)
      (if (Utilities|Array|IsNotEmpty (Variables|Default|GetIngredientIDs))
        (Development|PrintString (Utilities|String|ToString(Float) _returnvalue))
        (if (< _returnvalue _cookingtime) ; If Not finished cooking
          (Development|PrintString "Not finished cooking yet")
          (elif (>= _returnvalue (* _cookingtime 2.0)) ; If burnt
            ;[1 1 1] Replace these with adding recipe back into players inventory
            (Game|SpawnActorfromClass "/Game/Blueprints/Recipes/ARecipe_Burnt.ARecipe_Burnt_C" _returnvalue_4 "AlwaysSpawn" 0 0)
            (Utilities|Array|Clear (Variables|Default|GetIngredientIDs) :!label _label)
            (Variables|Default|SetbIsOn false)
            (Class|KismetSystemLibrary|PauseTimer 0 "FUNC")
            (elif (!= (Variables|Default|GetCreatedRecipeID) 0) ; If valid recipe
              (bind _asbp_arecipe (Utilities|Casting|CastToBP_ARecipeClass (Utilities|Array|Get(acopy) (Variables|Default|GetRecipeActors) (Variables|Default|GetCreatedRecipeID)))
                (:then
                  (if (== (Variables|Default|GetCreatedRecipeID) (.ID (Utilities|GetClassDefaults _asbp_arecipe)))
                    (Game|SpawnActorfromClass _asbp_arecipe _returnvalue_4 "AlwaysSpawn" 0 0)
                    (goto _label)))
                (:CastFailed
                  (Development|PrintString "Well fuck")))
              (else
                (Game|SpawnActorfromClass "/Game/Blueprints/Recipes/ARecipe_Wrong.ARecipe_Wrong_C" _returnvalue_4 "AlwaysSpawn" 0 0)
                (goto _label)))))
        (else
          (Development|PrintString "Nothing in there dumbass")
          (Variables|Default|SetbIsOn false)))
      (else
        (Utilities|Time|SetTimerbyFunctionName 0 "FUNC" 5e+02)
        (Variables|Default|SetbIsOn true)
        (if (Utilities|Array|IsNotEmpty (Variables|Default|GetIngredientIDs))
          ;[1 1 1] In theory this should work, can't test until inventory system is in place
          (bind _returnvalue_5 (Class|DataTableFunctionLibrary|GetDataTableColumnasString "/Game/Blueprints/DT_Objects.DT_Objects" "IngredientsID"))
          (for _array_element _returnvalue_5
            (for (_array_element_2 _array_index) (Utilities|String|ParseIntoArray _array_element " ")
              (if (not (== (Math|Conversions|ToInteger(Byte) _array_element_2) (Utilities|Array|Get(acopy) (Variables|Default|GetIngredientIDs) _array_index)))
                (Variables|Default|Settemp true)))
            (if (Variables|Default|Gettemp)
              (Variables|Default|Settemp false)
              (else
                (Variables|Default|SetCreatedRecipeID 0) ; change it to check for correct recipe
              ))))))))

(fn TimerFunc)

(fn AddItem
  (params (_Item :type S%20Inventory%20Item%20Structure))
  (|CallParentFunction _Item))

(fn Turnon
  (if (> (Utilities|Array|Length (Variables|Default|GetIngredientIDs)) 0)
    (|CallParentFunction)
    (bind _returnvalue (Audio|SpawnSoundatLocation "/Game/Art/Sound/A_Boiling.A_Boiling" "0, 0, 0" "0, 0, 0" 1.0 1.0 0.0 0 0))
    (Variables|Default|SetSoundPlaying _returnvalue)
    (bind _array_element (Utilities|Array|ForEachLoopwithBreak (Variables|Default|GetRecipes) :!label _label)
      (:LoopBody
        (bind _output_get (LocalVariables|Set_Item _array_element))
        (Development|PrintString (Utilities|String|ToString(Name) (.Name (Utilities|Struct|BreakS_Object _output_get))))
        (LocalVariables|Set_Correct true)
        (Utilities|Array|Clear (LocalVariables|Get_TmpCheckArray))
        (if (== (Utilities|Array|Length (.IngredientsID (Utilities|Struct|BreakS_Object _output_get))) (Utilities|Array|Length (Variables|Default|GetIngredientIDs))) ; check if amount of ingridients correct
          (for _index (range 0 (- (Utilities|Array|Length (.IngredientsID (Utilities|Struct|BreakS_Object _output_get))) 1)) ; for checking purposes create an array of values that will be the size of ingdients
            (Utilities|Array|Add (LocalVariables|Get_TmpCheckArray) false))
          (bind _index_2 (Utilities|FlowControl|ForLoopwithBreak 0 (- (Utilities|Array|Length (.IngredientsID (Utilities|Struct|BreakS_Object _output_get))) 1))
            (:LoopBody
              (LocalVariables|Set_I _index_2)
              (bind _index_3 (Utilities|FlowControl|ForLoopwithBreak 0 (- (Utilities|Array|Length (Variables|Default|GetIngredientIDs)) 1) :!label _label_2)
                (:LoopBody
                  (LocalVariables|Set_J _index_3)
                  (if (Utilities|Array|IsValidIndex (LocalVariables|Get_TmpCheckArray) (LocalVariables|Get_J)) ; if the ingridient was already checked and is correct - don't care
                    (if (not (Utilities|Array|Get(acopy) (LocalVariables|Get_TmpCheckArray) (LocalVariables|Get_J))) ; if the ingridient was already checked and is correct - don't care
                      (if (== (Utilities|Array|Get(acopy) (Variables|Default|GetIngredientIDs) (LocalVariables|Get_J)) (Utilities|Array|Get(acopy) (.IngredientsID (Utilities|Struct|BreakS_Object _output_get)) (LocalVariables|Get_I))) ; compare the ingridients
                        (Utilities|Array|SetArrayElem (LocalVariables|Get_TmpCheckArray) (LocalVariables|Get_J) true)
                        (goto _label_2 Break)))))))
            (:Completed
              (for _index_4 (range 0 (- (Utilities|Array|Length (LocalVariables|Get_TmpCheckArray)) 1))
                (if (not (Utilities|Array|Get(acopy) (LocalVariables|Get_TmpCheckArray) _index_4))
                  (LocalVariables|Set_Correct false)))
              (if (LocalVariables|Get_Correct)
                (goto _label Break))))))
      (:Completed
        (if (LocalVariables|Get_Correct)
          _
          (else
            ;[0.97 0 0] incorrect recipe
            (bind __item (CallFunction|FetchfromDatabase "IncorrectRecipe"))
            (LocalVariables|Set_Item __item)))
        ;[0.4028 1 0.3618] correct recipe
        (bind _output_get_2 (Variables|Default|SetProcessed%20Item (LocalVariables|Get_Item)))
        ;[1 1 1] Timer Start
        (bind _returnvalue_2 (Utilities|Time|SetTimerbyFunctionName 0 "TimerFunc" (.TimeToCook (Utilities|Struct|BreakS_Object _output_get_2))))
        (Variables|Default|SetTimerHandle _returnvalue_2)))))

(fn Retrieve
  (params (_ActiveTentacleID :type Integer))
  (bind _processed_item (Variables|Default|GetProcessed%20Item))
  (bind (_id _ingredientsid _toolsid _name _displayname _timetocook _timestart _timeend _placeholderforblueprint _rewardvalue _itemtype) (Utilities|Struct|BreakS_Object _processed_item))
  (return (Utilities|Struct|MakeS_InventoryItem _id _displayname _itemtype _ActiveTentacleID _name)))

(fn TurnOff
  (bind _timerhandle (Variables|Default|GetTimerHandle))
  (|CallParentFunction)
  (Audio|Components|Audio|FadeOut (Variables|Default|GetSoundPlaying) 1.0 0.0 "Linear" :!class /Script/Engine.AudioComponent)
  (Components|Activation|Deactivate (Variables|Default|GetSmokeConstant))
  (Components|Activation|Deactivate (Variables|Default|GetSmokeBurned))
  (if (Utilities|Time|IsTimerActivebyHandle _timerhandle)
    (Utilities|Time|ClearandInvalidateTimerbyHandle _timerhandle)))