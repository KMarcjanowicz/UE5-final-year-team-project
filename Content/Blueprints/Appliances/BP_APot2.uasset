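; Cooking pot appliance that takes ingredients from the player's tentacles and cooks them into a dish, collected with a bowl.
; On BeginPlay it loads its recipes from DT_Objects; TurnOn matches ingredients regardless of order, falling back to an incorrect-recipe result.
; An empty timer function serves as a clock that Tick polls for cooking, finished and burnt stages.
; These stages drive smoke, sound, tutorial dialogue and the player-facing inventory widget.
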(event Custom|OnEndCursorOver_Event
  (params (TouchedComponent :type Primitive%20Component%20Object%20Reference))
  (Rendering|SetVisibility (Variables|Default|GetInventoryWidget) false false)
  (Rendering|Material|SetScalarParameterValueonMaterials (Variables|Default|GetStaticMesh) "Selected" 0.0))

(event Custom|OnBeginCursorOver_Event
  (params (TouchedComponent :type Primitive%20Component%20Object%20Reference))
  (Rendering|SetVisibility (Variables|Default|GetInventoryWidget) true false)
  ;[1 1 1] turn off yellow highlight if it is on
  (if (not (Variables|Default|GetbIsOn))
    (Rendering|Material|SetScalarParameterValueonMaterials (Variables|Default|GetStaticMesh) "Selected" 1.0)))

(event EventBeginPlay
  (bind _staticmesh (Variables|Default|GetStaticMesh))
  (|CallParentFunction)
  (EventDispatchers|BindEventtoOnEndCursorOver _staticmesh (delegate Custom|OnEndCursorOver_Event))
  (EventDispatchers|AssignOnBeginCursorOver _staticmesh (delegate Custom|OnBeginCursorOver_Event))
  ;[1 0.6249 0] Pot inventory
  (bind _aswb_pot_inventory (Utilities|Casting|CastToWB_PotInventory (UserInterface|GetWidget (Variables|Default|GetInventoryWidget))))
  (Variables|Default|SetPot%20Inventory _aswb_pot_inventory)
  ;[1 1 1] Get the recipes from the data table
  (bind _outrownames (DataTable|GetDataTableRowNames "/Game/Blueprints/DT_Objects.DT_Objects"))
  (for _array_element _outrownames
    (bind _returnvalue (Utilities|GetDataTableRow "/Game/Blueprints/DT_Objects.DT_Objects" _array_element)
      (:then
        (if (and (Utilities|Enum|Equal(Enum) (.ItemType (Utilities|Struct|BreakS_Object _returnvalue)) "NewEnumerator2") (Utilities|Enum|Equal(Enum) (.ApplianceType (Utilities|Struct|BreakS_Object _returnvalue)) "NewEnumerator0"))
          (Utilities|Array|Add (Variables|Default|GetRecipes) _returnvalue))))))

(event MouseInput|EventActorEndCursorOver)

(event EventTick
  (params (DeltaSeconds :type Float%20%28single-precision%29))
  (bind _returnvalue (Class|KismetSystemLibrary|GetTimerElapsedTime 0 "TimerFunc"))
  (bind _bp_dialogue (Variables|Default|GetBP_Dialogue))
  ;[1 0.8386 0] rotate inventory widget towards camera
  (Transformation|SetWorldRotation (Variables|Default|GetInventoryWidget) (Math|Rotator|FindLookatRotation (Transformation|GetActorLocation) (Transformation|GetActorLocation (Game|Player|GetPlayerPawn 0))) false false)
  ;[1 1 1] this doesn't work - after putting in correct times
  (if (Variables|Default|GetbIsOn)
    (if (> _returnvalue (* (Variables|Default|GetCookingTime) 2.0)) ; If food is burnt, play burnt smoke
      (Utilities|FlowControl|DoOnce false
        (:Completed
          (Components|Activation|Activate (Variables|Default|GetSmokeFinish) false)
          (bind _returnvalue_2 (Audio|SpawnSoundatLocation (Variables|Default|GetBurningSound) "0, 0, 0" "0, 0, 0" 1.0 1.0 0.0 0 0))
          (Audio|Components|Audio|FadeOut (Variables|Default|GetSoundPlaying) 0.2 0.0 "Linear" :!class /Script/Engine.AudioComponent)
          (Variables|Default|SetSoundPlaying _returnvalue_2)
          (Components|Activation|Deactivate (Variables|Default|GetSmokeConstant))
          (Components|Activation|Activate (Variables|Default|GetSmokeBurned) false)
          (if (Variables|Default|GetIfcookedburnt)
            _
            (else
              ;[1 1 1] Tutorial
              (Class|BPITutorial|CookBurnt-Dialouge(Message) _bp_dialogue)
              (Variables|Default|SetIfcookedburnt true)))
          ;[0.1823 0.07252 0] food burnt
          (bind __item (CallFunction|FetchfromDatabase "BurntRecipeBowl"))
          (Variables|Default|SetProcessed%20Item __item)))
      (elif (and (> _returnvalue (Variables|Default|GetCookingTime)) (not (Variables|Default|GetbHoldsProcessedItem))) ; If food is cooked play big smoke
        (Utilities|FlowControl|DoOnce false :!label _label
          (:Completed
            (Components|Activation|Activate (Variables|Default|GetSmokeFinish) false)
            (if (Variables|Default|GetIfcookedfinished)
              _
              (else
                (Class|BPITutorial|CookFinished-Dialouge(Message) _bp_dialogue)
                (Variables|Default|SetIfcookedfinished true)))
            ;[1 0.7854 0] UI food finish
            (Default|MakeVisibleCanvas (Variables|Default|GetPot%20Inventory) 3)))
        (else
          (Utilities|FlowControl|DoOnce false :!label _label_2
            (:Completed
              (Components|Activation|Activate (Variables|Default|GetSmokeConstant) false) ; If food is cooking but not yet done play small smoke
              (if (Variables|Default|GetIfcookedstart)
                (goto _label Reset)
                (else
                  (Class|BPITutorial|CookStart-Dialouge(Message) _bp_dialogue)
                  (Variables|Default|SetIfcookedstart true)
                  (goto _label Reset))))))))
    (bind _newparam (Default|GetFoodFinishImage (Variables|Default|GetPot%20Inventory)))
    (Default|SetInventorySlotImage (Variables|Default|GetPot%20Inventory) _newparam (.DisplayName (Utilities|Struct|BreakS_Object (Variables|Default|GetProcessed%20Item))))
    (Variables|Default|SetbHoldsProcessedItem true)
    (Utilities|Array|Clear (Variables|Default|GetIngredientIDs))
    (else
      (Components|Activation|Deactivate (Variables|Default|GetSmokeConstant))
      (Components|Activation|Deactivate (Variables|Default|GetSmokeBurned))
      (goto _label_2 Reset))))

(event MouseInput|EventActorBeginCursorOver)

(event EventInteract
  (params (_Tentacle :type S%20Tentacle%20Structure) (_Item :type S%20Inventory%20Item%20Structure))
  (bind (_tentacleid _bisbusy) (Utilities|Struct|BreakS_Tentacle _Tentacle))
  (bind (_id _displayname _type) (Utilities|Struct|BreakS_InventoryItem _Item))
  (if (and (and _bisbusy (> _id 0)) (Utilities|Enum|Equal(Enum) _type "NewEnumerator1")) ; check if holding item and if item is default
    (if (not (Variables|Default|GetbIsOn)) ; check if the appliance is running
      (CallFunction|Fetch _Item)
      (bind _asbp_first_person_character (Utilities|Casting|CastToBP_FirstPersonCharacter (Game|Player|GetPlayerPawn 0)))
      (Default|PlayAnim _asbp_first_person_character 11)
      ;[1 1 1] this doesn't work - after putting in correct times
      (Utilities|FlowControl|DoOnce false) ; enters at Reset
    )
    (elif (not (and (== (.ID (Utilities|Struct|BreakS_InventoryItem _Item)) -1) (.bIsBusy (Utilities|Struct|BreakS_Tentacle _Tentacle)))) ; Check if tentacle is busy using other appliance
      (if (Variables|Default|GetbHoldsProcessedItem) ; check if there was something that cooked
        (bind __bisable (CallFunction|CheckifAblePickUp _tentacleid))
        ;[1 1 1] getting an item out
        (if (and __bisable (not (Variables|Default|GetbIsOn)))
          (bind __inventoryitem (CallFunction|Retrieve _tentacleid))
          (bind _asbp_first_person_character_2 (Utilities|Casting|CastToBP_FirstPersonCharacter (Game|Player|GetPlayerPawn 0)))
          (Default|PlayAnim _asbp_first_person_character_2 17)
          (Default|AddItem (Variables|/Game/Blueprints/Actor/BP_FirstPersonCharacter.BP_FirstPersonCharacter_C|GetBP_AC_Inventory _asbp_first_person_character_2) (.DisplayName (Utilities|Struct|BreakS_InventoryItem __inventoryitem)) _tentacleid (.ID (Utilities|Struct|BreakS_InventoryItem __inventoryitem)) (.Type (Utilities|Struct|BreakS_InventoryItem __inventoryitem)) (.DatabaseReferenceName (Utilities|Struct|BreakS_InventoryItem __inventoryitem)))
          (CallFunction|NewRecipeLearnt? (.DatabaseReferenceName (Utilities|Struct|BreakS_InventoryItem __inventoryitem)))
          (Default|SetTentacleBusy _asbp_first_person_character_2 _tentacleid)
          (Variables|Default|SetbHoldsProcessedItem false)
          ;[1 0.8177 0] UI reset
          (Default|ClearApplianceInventory (Variables|Default|GetPot%20Inventory))
          (Default|MakeVisibleCanvas (Variables|Default|GetPot%20Inventory) 1))))))

(fn ConstructionScript
  (|CallParentFunction)
  (Variables|Default|SetbIsActiveAppliance false)
  (Variables|Default|SetIngredientCap 6)
  (Variables|Default|SetType "NewEnumerator4")
  (Variables|Default|SetName "Pot")
  (Rendering|SetVisibility (Variables|Default|GetInventoryWidget) false false))

(fn TimerFunc)

(fn AddItem
  (params (_Item :type S%20Inventory%20Item%20Structure))
  (|CallParentFunction _Item)
  ;[1 0.9174 0] Add item to UI
  (Default|DisplayItem (Variables|Default|GetPot%20Inventory) (.DisplayName (Utilities|Struct|BreakS_InventoryItem _Item))))

(fn Turnon
  (if (> (Utilities|Array|Length (Variables|Default|GetIngredientIDs)) 0)
    (|CallParentFunction)
    ;[1 0.9108 0] inventory UI
    (Default|MakeVisibleCanvas (Variables|Default|GetPot%20Inventory) 2)
    (Default|ClearApplianceInventory (Variables|Default|GetPot%20Inventory))
    (bind _asbp_first_person_character (Utilities|Casting|CastToBP_FirstPersonCharacter (Game|Player|GetPlayerPawn 0)))
    (Default|PlayAnim _asbp_first_person_character 10)
    (bind _returnvalue (Audio|SpawnSoundatLocation "/Game/Art/Sound/A_Boiling.A_Boiling" "0, 0, 0" "0, 0, 0" 1.0 1.0 0.0 0 0))
    (Variables|Default|SetSoundPlaying _returnvalue)
    (bind _array_element (Utilities|Array|ForEachLoopwithBreak (Variables|Default|GetRecipes) :!label _label)
      (:LoopBody
        (bind _output_get (LocalVariables|Set_Item _array_element))
        (LocalVariables|Set_Correct true)
        (Utilities|Array|Clear (LocalVariables|Get_TmpCheckArray))
        (if (== (Utilities|Array|Length (.IngredientsID (Utilities|Struct|BreakS_Object _output_get))) (Utilities|Array|Length (Variables|Default|GetIngredientIDs))) ; check if amount of ingridients correct
          (for _index (range 0 (- (Utilities|Array|Length (.IngredientsID (Utilities|Struct|BreakS_Object _output_get))) 1)) ; for checking purposes create an array of values that will be the size of ingdients
            (Utilities|Array|Add (LocalVariables|Get_TmpCheckArray) false))
          (bind _index_2 (Utilities|FlowControl|ForLoopwithBreak 0 (- (Utilities|Array|Length (.IngredientsID (Utilities|Struct|BreakS_Object _output_get))) 1))
            (:LoopBody
              (LocalVariables|Set_I _index_2)
              (bind _index_3 (Utilities|FlowControl|ForLoopwithBreak 0 (- (Utilities|Array|Length (Variables|Default|GetIngredientIDs)) 1) :!label _label_2)
                (:LoopBody
                  (LocalVariables|Set_J _index_3)
                  (if (Utilities|Array|IsValidIndex (LocalVariables|Get_TmpCheckArray) (LocalVariables|Get_J)) ; check if valid index
                    (if (not (Utilities|Array|Get(acopy) (LocalVariables|Get_TmpCheckArray) (LocalVariables|Get_J))) ; if the ingridient was already checked and is correct - don't care
                      (if (== (Utilities|Array|Get(acopy) (Variables|Default|GetIngredientIDs) (LocalVariables|Get_J)) (Utilities|Array|Get(acopy) (.IngredientsID (Utilities|Struct|BreakS_Object _output_get)) (LocalVariables|Get_I))) ; compare the ingridients
                        (Utilities|Array|SetArrayElem (LocalVariables|Get_TmpCheckArray) (LocalVariables|Get_J) true)
                        (goto _label_2 Break)
                        (else
                          (Utilities|Array|SetArrayElem (LocalVariables|Get_TmpCheckArray) (LocalVariables|Get_J) false)
                          (Development|PrintString "false ing"))))))))
            (:Completed
              (for _index_4 (range 0 (- (Utilities|Array|Length (LocalVariables|Get_TmpCheckArray)) 1))
                (if (not (Utilities|Array|Get(acopy) (LocalVariables|Get_TmpCheckArray) _index_4))
                  (LocalVariables|Set_Correct false)))
              (if (LocalVariables|Get_Correct)
                (goto _label Break))))
          (else
            ;[1 0 0.006631] important
            (LocalVariables|Set_Correct false))))
      (:Completed
        (if (LocalVariables|Get_Correct)
          _
          (else
            ;[0.97 0 0] incorrect recipe
            (bind __item (CallFunction|FetchfromDatabase "IncorrectRecipeBowl"))
            (LocalVariables|Set_Item __item)))
        ;[0.4028 1 0.3618] correct recipe
        (bind _output_get_2 (Variables|Default|SetProcessed%20Item (LocalVariables|Get_Item)))
        ;[1 1 1] Timer Start
        (bind _returnvalue_2 (Utilities|Time|SetTimerbyFunctionName 0 "TimerFunc" (* (.TimeToCook (Utilities|Struct|BreakS_Object _output_get_2)) 3.0)))
        (Variables|Default|SetTimerHandle _returnvalue_2)
        (Variables|Default|SetCookingTime (.TimeToCook (Utilities|Struct|BreakS_Object _output_get_2)))))))

(fn Retrieve
  (params (_ActiveTentacleID :type Integer))
  (bind _processed_item (Variables|Default|GetProcessed%20Item))
  (bind (_id _ingredientsid _name _displayname _timetocook _rewardvalue _itemtype) (Utilities|Struct|BreakS_Object _processed_item))
  (return (Utilities|Struct|MakeS_InventoryItem _id _displayname _itemtype _ActiveTentacleID _name)))

(fn TurnOff
  (bind _timerhandle (Variables|Default|GetTimerHandle))
  (|CallParentFunction)
  (bind _asbp_first_person_character (Utilities|Casting|CastToBP_FirstPersonCharacter (Game|Player|GetPlayerPawn 0)))
  (Default|PlayAnim _asbp_first_person_character 20)
  (Audio|Components|Audio|FadeOut (Variables|Default|GetSoundPlaying) 1.0 0.0 "Linear" :!class /Script/Engine.AudioComponent)
  (Components|Activation|Deactivate (Variables|Default|GetSmokeConstant))
  (Components|Activation|Deactivate (Variables|Default|GetSmokeBurned))
  (if (Utilities|Time|IsTimerActivebyHandle _timerhandle)
    (Utilities|Time|ClearandInvalidateTimerbyHandle _timerhandle)))

(fn CheckifAblePickUp
  (params (_TentacleID :type Integer))
  (bind _asbp_first_person_character (Utilities|Casting|CastToBP_FirstPersonCharacter (Game|Player|GetPlayerPawn 0)))
  (bind __item (Default|GetItem (Variables|/Game/Blueprints/Actor/BP_FirstPersonCharacter.BP_FirstPersonCharacter_C|GetBP_AC_Inventory _asbp_first_person_character) _TentacleID))
  (if (and (Utilities|Enum|Equal(Enum) (.Type (Utilities|Struct|BreakS_InventoryItem __item)) "NewEnumerator0") (== (.DatabaseReferenceName (Utilities|Struct|BreakS_InventoryItem __item)) "Bowl"))
    (return true)))

(fn GetPassScore
  (return 0.0))

(fn StoveOff-Dialouge)