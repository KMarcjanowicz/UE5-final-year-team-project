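; Cooking pot appliance that turns the ingredients placed in it into a recipe actor.
; When on and filled, Tick switches it off, starts smoke and waits CookingTime.
; It compares ingredient IDs index by index against each entry in Recipes, so order matters, and keeps the last match.
; The BP_ARecipe class with the matching ID spawns beside the pot; the cleanup clears ingredients and pulses finish smoke, even without a match.
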(event EventTick
  (params (DeltaSeconds :type Float%20%28single-precision%29))
  (bind _recipes (Variables|Default|GetRecipes))
  (bind _smokefinish (Variables|Default|GetSmokeFinish))
  ;[1 1 1] Check if the ingredients in the appliance match any recipes in that appliances recipe list
  (|CallParentFunction DeltaSeconds)
  (if (Variables|Default|GetisOn)
    (if (Utilities|Array|IsNotEmpty (Variables|Default|GetIngredientIDs))
      (Variables|Default|SetisOn false)
      (Components|Activation|Activate (Variables|Default|GetSmokeConstant) false)
      (Utilities|FlowControl|Delay (Variables|Default|GetCookingTime))
      (for (_ _array_index) _recipes ; For each recipe the appliance can create
        (bind (_array_element _array_index_2) (Utilities|Array|ForEachLoopwithBreak (.IngredientsID (Utilities|Struct|BreakSRecipe (Utilities|Array|Get(acopy) _recipes _array_index)))) ; For each ingredient in the recipe
          (:LoopBody
            (if (not (== _array_element (Utilities|Array|Get(acopy) (Variables|Default|GetIngredientIDs) _array_index_2)))
              (Variables|Default|Settemp true)
              (Development|PrintString "No work")))
          (:Completed
            (if (Variables|Default|Gettemp)
              (Variables|Default|Settemp false)
              (else
                (bind _output_get (Variables|Default|SetCreatedRecipeID (.ID (Utilities|Struct|BreakSRecipe (Utilities|Array|Get(acopy) _recipes _array_index)))))
                (Development|PrintString "Recipe created:")
                (Development|PrintString (Utilities|String|ToString(Integer) _output_get)))))))
      (if (!= (Variables|Default|GetCreatedRecipeID) 0)
        (Development|PrintString "New RECIPE")
        (Variables|Default|SetisOn false)
        (for _array_element_2 0
          (bind _asbp_arecipe (Utilities|Casting|CastToBP_ARecipeClass _array_element_2)
            (:then
              (if (== (Variables|Default|GetCreatedRecipeID) (Utilities|GetClassDefaults _asbp_arecipe))
                (Game|SpawnActorfromClass _asbp_arecipe (Math|Conversions|ToTransform(Vector) (+ (Transformation|GetActorLocation) "0,200.000000,50.000000")) "AlwaysSpawn" 0 0))
              (Utilities|Array|Clear (Variables|Default|GetIngredientIDs))
              (Components|Activation|Deactivate (Variables|Default|GetSmokeConstant))
              (Utilities|FlowControl|Delay 0.2)
              (Components|Activation|Activate _smokefinish false)
              (Utilities|FlowControl|Delay 0.1)
              (Components|Activation|Deactivate _smokefinish))
            (:CastFailed
              (Development|PrintString "Well fuck"))))
        (if (== (Variables|Default|GetCreatedRecipeID) (Utilities|GetClassDefaults _asbp_arecipe))
          (Game|SpawnActorfromClass _asbp_arecipe (Math|Conversions|ToTransform(Vector) (+ (Transformation|GetActorLocation) "0,200.000000,50.000000")) "AlwaysSpawn" 0 0))
        (else
          (Development|PrintString "No recipes")))
      (Utilities|Array|Clear (Variables|Default|GetIngredientIDs))
      (Components|Activation|Deactivate (Variables|Default|GetSmokeConstant))
      (Utilities|FlowControl|Delay 0.2)
      (Components|Activation|Activate _smokefinish false)
      (Utilities|FlowControl|Delay 0.1)
      (Components|Activation|Deactivate _smokefinish))))

(fn ConstructionScript
  (|CallParentFunction))