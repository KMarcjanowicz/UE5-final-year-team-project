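; Cutting board appliance that turns an ingredient into a recipe result using a tool.
; When it holds both, Tick swaps in a temporary working material, waits the cooking time, then searches its recipes by tool ID and first ingredient ID only.
; A match spawns the corresponding ingredient actor beside the board.
; After a spawn or failed match, it clears its inputs and swaps the material back.
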(event EventTick
  (params (DeltaSeconds :type Float%20%28single-precision%29))
  (bind _recipes (Variables|Default|GetRecipes))
  (bind _ingredientids (Variables|Default|GetIngredientIDs))
  (bind _output (Utilities|Array|Get(acopy) _ingredientids))
  ;[1 1 1] Check if the ingredients in the appliance match any recipes in that appliances recipe list
  (if (Utilities|Array|IsNotEmpty (Variables|Default|GetIngredientIDs))
    (if (!= (Variables|Default|GetToolID) 0)
      (Rendering|Material|SetMaterial (Variables|Default|GetStaticMesh) 0 "/Game/StarterContent/Materials/M_Concrete_Grime.M_Concrete_Grime") ; Temp change material., change this to look like it's on later
      (Utilities|FlowControl|Delay (Variables|Default|GetCookingTime))
      (for (_ _array_index) _recipes ; For each recipe the appliance can create
        (for _array_element (.ToolsID (Utilities|Struct|BreakSRecipe (Utilities|Array|Get(acopy) _recipes _array_index))) ; Check each tool that can be used to see if the selected one is valid
          (Development|PrintString (Utilities|String|ToString(Integer) _array_element))
          (if (== _array_element (Variables|Default|GetToolID))
            (Variables|Default|SetValidTool (== _array_element (Variables|Default|GetToolID)))))
        (if (Variables|Default|GetValidTool)
          (for _array_element_2 (.IngredientsID (Utilities|Struct|BreakSRecipe (Utilities|Array|Get(acopy) _recipes _array_index))) ; If there is a valid tool, check  what the ingredient turns into
            (Development|PrintString (Utilities|String|ToString(Integer) _output))
            (if (== _array_element_2 _output)
              (Variables|Default|SetCreatedRecipeID (.ID (Utilities|Struct|BreakSRecipe (Utilities|Array|Get(acopy) _recipes _array_index))))))))
      (if (!= (Variables|Default|GetCreatedRecipeID) 0)
        (Development|PrintString "New RECIPE")
        (for _array_element_3 (Variables|Default|GetRecipeActors)
          (bind _asbp_aingredient (Utilities|Casting|CastToBP_AIngredientClass _array_element_3))
          (if (== (Variables|Default|GetCreatedRecipeID) (.ID (Utilities|GetClassDefaults _asbp_aingredient)))
            (Game|SpawnActorfromClass _asbp_aingredient (Math|Conversions|ToTransform(Vector) (+ (Transformation|GetActorLocation) "0,200.000000,50.000000")) "AlwaysSpawn" 0 0)
            (Utilities|Array|Clear (Variables|Default|GetIngredientIDs))
            (Variables|Default|SetToolID 0)
            (Rendering|Material|SetMaterial (Variables|Default|GetStaticMesh) 0 "/Game/StarterContent/Materials/M_Ceramic_Tile_Checker.M_Ceramic_Tile_Checker")))
        (else
          (Development|PrintString "No recipes")
          (Utilities|Array|Clear (Variables|Default|GetIngredientIDs))
          (Variables|Default|SetToolID 0)
          (Rendering|Material|SetMaterial (Variables|Default|GetStaticMesh) 0 "/Game/StarterContent/Materials/M_Ceramic_Tile_Checker.M_Ceramic_Tile_Checker"))))))

(fn ConstructionScript
  (|CallParentFunction))