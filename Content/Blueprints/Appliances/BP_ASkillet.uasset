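; Skillet cooking appliance that takes up to three ingredients, shown on mesh sockets, and occupies the player's active tentacle while cooking.
; On BeginPlay it caches recipes and cookable foods from DT_Objects; one ingredient becomes its cooked version, several must match a recipe in order or yield IncorrectRecipe.
; An empty timer serves as a stopwatch polled on Tick to swap in the result and free the tentacle.
; Pickup checks for a plate.
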(event Collision|EventActorBeginOverlap
  (params (OtherActor :type Actor%20Object%20Reference))
  (|CallParentFunction OtherActor) ; This node is disabled and will not be called.\nDrag off pins to build functionality.
)

(event EventTick
  (params (DeltaSeconds :type Float%20%28single-precision%29))
  (bind _returnvalue (Class|KismetSystemLibrary|GetTimerElapsedTime 0 "TimerFunc"))
  (|CallParentFunction DeltaSeconds)
  (if (> _returnvalue (* 1.5 (Variables|Default|GetCookingTime)))
    (Development|PrintString "Food burnt")
    (elif (and (>= _returnvalue (Variables|Default|GetCookingTime)) (not (Variables|Default|GetbHoldsProcessedItem)))
      (Development|PrintString "Puff smoke - meal ready")
      (CallFunction|CookingTimerFinish))))

(event EventBeginPlay
  ;[1 1 1] Get the recipes from the data table
  (bind _outrownames (DataTable|GetDataTableRowNames "/Game/Blueprints/DT_Objects.DT_Objects"))
  (for _array_element _outrownames
    (bind _returnvalue (Utilities|GetDataTableRow "/Game/Blueprints/DT_Objects.DT_Objects" _array_element)
      (:then
        (if (and (Utilities|Enum|Equal(Enum) (.ItemType (Utilities|Struct|BreakS_Object _returnvalue)) "NewEnumerator2") (Utilities|Enum|Equal(Enum) (.ApplianceType (Utilities|Struct|BreakS_Object _returnvalue)) "NewEnumerator1"))
          (Utilities|Array|Add (Variables|Default|GetRecipes) _returnvalue)
          (elif (> (Utilities|String|FindSubstring (Utilities|String|ToString(Name) (.Processed (Utilities|Struct|BreakS_Object _returnvalue))) "Cooked") -1)
            (Utilities|Array|Add (Variables|Default|GetFoodToProcess) _returnvalue)))))))

(fn ConstructionScript
  (|CallParentFunction)
  (Variables|Default|SetbIsActiveAppliance true)
  (Variables|Default|SetType "NewEnumerator4")
  (Variables|Default|SetIngredientCap 3)
  (Variables|Default|SetName "Skillet")
  (Utilities|Array|Clear (Variables|Default|GetSockets))
  (for _array_element (Transformation|GetAllSocketNames (Variables|Default|GetStaticMesh))
    (Utilities|Array|Add (Variables|Default|GetSockets) (Utilities|Struct|MakeS_Socket _array_element false))))

(fn Turnon
  (if (> (Utilities|Array|Length (Variables|Default|GetIngredientIDs)) 0) ; check if not empty
    (|CallParentFunction)
    ;[0.2993 0.8699 1] Set tentacle using this appliance as busy
    (bind __activetentacle (Class|BPIPlayerController|ActiveTentacle(Message) (Game|GetPlayerController 0)))
    (Variables|Default|SetUsingTentacleID __activetentacle)
    (bind _asbp_first_person_character (Utilities|Casting|CastToBP_FirstPersonCharacter (Game|Player|GetPlayerPawn 0)))
    (Default|SetTentacleBusy _asbp_first_person_character __activetentacle)
    (Development|PrintString (Utilities|String|Append (Utilities|String|ToString(Integer) __activetentacle) " was set to busy"))
    (Default|AddItem (Variables|/Game/Blueprints/Actor/BP_FirstPersonCharacter.BP_FirstPersonCharacter_C|GetBP_AC_Inventory _asbp_first_person_character) "x" __activetentacle -1 "NewEnumerator1" "N/A") ; temp item to show that tentacle busy
    (if (== (Utilities|Array|Length (Variables|Default|GetIngredientIDs)) 1) ; check if for cooking or processing an item
      (Development|PrintString "Cooking one item")
      (CallFunction|SingleItemProccessing)
      (else
        (Development|PrintString "Multiple items into recipe")
        (CallFunction|MultipleItemsCooking)))))

(fn AddItem
  (params (_Item :type S%20Inventory%20Item%20Structure))
  (bind __item (CallFunction|FetchfromDatabase (.DatabaseReferenceName (Utilities|Struct|BreakS_InventoryItem _Item))))
  (|CallParentFunction _Item)
  (CallFunction|AttachItem (.Placeholderforblueprint (Utilities|Struct|BreakS_Object __item)) (- (Utilities|Array|Length (Variables|Default|GetIngredientIDs)) 1)))

(fn AttachItem
  (params (_Class :type BP%20A%20Interactable%20Item%20Class%20Reference) (_Socket :type Integer))
  (bind _sockets (Variables|Default|GetSockets))
  (bind _output (Utilities|Array|Get(acopy) _sockets _Socket))
  (bind (_name _bisoccupied) (Utilities|Struct|BreakS_Socket _output))
  (LocalVariables|SetSocket _Socket)
  (if (not _bisoccupied)
    (bind _returnvalue (Game|SpawnActorfromClass _Class (Transformation|GetSocketTransform (Variables|Default|GetStaticMesh) _name "RTS_World") "AlwaysSpawn" 0 0))
    (Physics|SetSimulatePhysics (Variables|/Game/Blueprints/BP_AInteractableItem.BP_AInteractableItem_C|GetStaticMesh _returnvalue) false)
    (Transformation|AttachComponentToComponent _returnvalue (Variables|Default|GetStaticMesh) _name "KeepRelative" "KeepRelative" "KeepRelative" true)
    (Class|BPIPickUp|SetinUse(Message) _returnvalue true)
    (Utilities|Array|SetArrayElem (Variables|Default|GetSockets) (LocalVariables|GetSocket) (Utilities|Struct|MakeS_Socket _name true))
    ;[1 1 1] add actor to be destoryed when finished cooking
    (Utilities|Array|Add (Variables|Default|GetActorsToDestroy) _returnvalue)))

(fn SingleItemProccessing
  (Variables|Default|SetbHoldsProcessedItem false)
  (Variables|Default|SetbIsOn true)
  (bind _array_element (Utilities|Array|ForEachLoopwithBreak (Variables|Default|GetFoodToProcess) :!label _label)
    (:LoopBody
      (bind _output_get (LocalVariables|Set_Item _array_element))
      (if (== (.ID (Utilities|Struct|BreakS_Object _output_get)) (Utilities|Array|Get(acopy) (Variables|Default|GetIngredientIDs)))
        (LocalVariables|Set_ItemName (.Processed (Utilities|Struct|BreakS_Object _output_get)))
        (goto _label Break)))
    (:Completed
      (bind _returnvalue (Utilities|GetDataTableRow "/Game/Blueprints/DT_Objects.DT_Objects" (LocalVariables|Get_ItemName))
        (:then
          (Variables|Default|SetProcessed%20Item _returnvalue)
          (bind _returnvalue_2 (Utilities|Time|SetTimerbyFunctionName 0 "TimerFunc" (* (.TimeToCook (Utilities|Struct|BreakS_Object (LocalVariables|Get_Item))) 3.0)))
          (Variables|Default|SetTimerHandle _returnvalue_2)
          (Variables|Default|SetCookingTime (.TimeToCook (Utilities|Struct|BreakS_Object (LocalVariables|Get_Item)))))))))

(fn MultipleItemsCooking
  (Variables|Default|SetbHoldsProcessedItem false)
  (LocalVariables|Set_Correct false)
  (bind _array_element (Utilities|Array|ForEachLoopwithBreak (Variables|Default|GetRecipes) :!label _label)
    (:LoopBody
      (if (LocalVariables|Get_Correct)
        (goto _label Break)
        (else
          (bind _output_get (LocalVariables|Set_Item _array_element))
          (LocalVariables|Set_Correct true)
          (if (== (Utilities|Array|Length (.IngredientsID (Utilities|Struct|BreakS_Object _output_get))) (Utilities|Array|Length (Variables|Default|GetIngredientIDs))) ; check if amount of ingridients correct
            (bind _index (Utilities|FlowControl|ForLoopwithBreak 0 (- (Utilities|Array|Length (.IngredientsID (Utilities|Struct|BreakS_Object _output_get))) 1))
              (:LoopBody
                (if (not (== (Utilities|Array|Get(acopy) (Variables|Default|GetIngredientIDs) _index) (Utilities|Array|Get(acopy) (.IngredientsID (Utilities|Struct|BreakS_Object _output_get)) _index)))
                  (LocalVariables|Set_Correct false))))
            (else
              (LocalVariables|Set_Correct false))))))
    (:Completed
      (if (LocalVariables|Get_Correct)
        _
        (else
          ;[0.97 0 0] incorrect recipe
          (bind __item (CallFunction|FetchfromDatabase "IncorrectRecipe"))
          (LocalVariables|Set_Item __item)))
      ;[0.4028 1 0.3618] correct recipe
      (bind _output_get_2 (Variables|Default|SetProcessed%20Item (LocalVariables|Get_Item)))
      (bind _returnvalue (Utilities|Time|SetTimerbyFunctionName 0 "TimerFunc" (* (.TimeToCook (Utilities|Struct|BreakS_Object _output_get_2)) 3.0)))
      (Variables|Default|SetTimerHandle _returnvalue)
      (Variables|Default|SetCookingTime (.TimeToCook (Utilities|Struct|BreakS_Object _output_get_2))))))

(fn TimerFunc
  ;[1 1 1] doesn't do anything - just for timers
)

(fn DetachItems
  (for (_array_element _array_index) (Variables|Default|GetActorsToDestroy)
    (Actor|DestroyActor _array_element)
    (Utilities|Array|SetArrayElem (Variables|Default|GetSockets) _array_index (Utilities|Struct|MakeS_Socket (.Name (Utilities|Struct|BreakS_Socket (Utilities|Array|Get(acopy) (Variables|Default|GetSockets) _array_index))) false)))
  (Utilities|Array|Clear (Variables|Default|GetActorsToDestroy)))

(fn Retrieve
  (params (_ActiveTentacleID :type Integer))
  (bind _processed_item (Variables|Default|GetProcessed%20Item))
  (bind (_id _ingredientsid _name _displayname _timetocook _placeholderforblueprint _rewardvalue _itemtype) (Utilities|Struct|BreakS_Object _processed_item))
  (Variables|Default|SetbHoldsProcessedItem false)
  (Variables|Default|SetbIsOn false)
  (CallFunction|DetachItems)
  (return (Utilities|Struct|MakeS_InventoryItem _id _displayname _itemtype _ActiveTentacleID _name)))

(fn CookingTimerFinish
  (bind _usingtentacleid (Variables|Default|GetUsingTentacleID))
  ;[1 1 1] timers
  (CallFunction|DetachItems)
  (CallFunction|AttachItem (.Placeholderforblueprint (Utilities|Struct|BreakS_Object (Variables|Default|GetProcessed%20Item))) 3)
  (Variables|Default|SetbHoldsProcessedItem true)
  (Utilities|Array|Clear (Variables|Default|GetIngredientIDs))
  (Utilities|Time|ClearandInvalidateTimerbyHandle (Variables|Default|GetTimerHandle))
  ;[0.577 0.93 1] free the tentacle
  (bind _asbp_first_person_character (Utilities|Casting|CastToBP_FirstPersonCharacter (Game|Player|GetPlayerPawn 0)))
  (Default|SetTentacleFree _asbp_first_person_character _usingtentacleid)
  (bind _asbp_first_person_game_mode (Utilities|Casting|CastToBP_FirstPersonGameMode (Game|GetGameMode)))
  (Default|DisplayObjectinTentacleHUD _asbp_first_person_game_mode (Utilities|Struct|MakeS_InventoryItem 0 "." "NewEnumerator11" _usingtentacleid) false))

(fn CheckifAblePickUp
  (params (_TentacleID :type Integer))
  (bind _asbp_first_person_character (Utilities|Casting|CastToBP_FirstPersonCharacter (Game|Player|GetPlayerPawn 0)))
  (bind __item (Default|GetItem (Variables|/Game/Blueprints/Actor/BP_FirstPersonCharacter.BP_FirstPersonCharacter_C|GetBP_AC_Inventory _asbp_first_person_character) _TentacleID))
  (if (and (Utilities|Enum|Equal(Enum) (.Type (Utilities|Struct|BreakS_InventoryItem __item)) "NewEnumerator0") (== (.DatabaseReferenceName (Utilities|Struct|BreakS_InventoryItem __item)) "Plate"))
    (return true)))