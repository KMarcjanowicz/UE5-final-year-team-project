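; Base cooking appliance Blueprint that the player's tentacles load with ingredients, start and empty.
; Interact either stores the held item's ID up to a cap, signals the appliance on, or hands the processed item to a free active tentacle.
; Retrieving an item records new recipes in the save slot and shows a popup when one is learnt.
; A widget shows contents and status on cursor hover; TimerFinished is an empty stub.
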(event EventTimer
  (params (_Seconds :type Float%20%28double-precision%29))
  (Utilities|FlowControl|Delay _Seconds)
  (Development|PrintString "timer finish")
  (CallFunction|TimerFinished))

(event MouseInput|EventActorBeginCursorOver
  (|CallParentFunction)
  (Rendering|SetVisibility (Variables|Default|GetInventoryWidget) true false))

(event MouseInput|EventActorEndCursorOver
  (|CallParentFunction)
  (Rendering|SetVisibility (Variables|Default|GetInventoryWidget) false false))

(event EventInteract
  (params (_Tentacle :type S%20Tentacle%20Structure) (_Item :type S%20Inventory%20Item%20Structure))
  (bind (_id _displayname) (Utilities|Struct|BreakS_InventoryItem _Item))
  (bind (_tentacleid _bisbusy) (Utilities|Struct|BreakS_Tentacle _Tentacle))
  (bind (_id_2 _displayname_2 _type) (Utilities|Struct|BreakS_InventoryItem _Item))
  (bind _popupwidgetreference (Variables|Default|GetPopupWidgetReference))
  (if (and (and _bisbusy (> _id_2 0)) (Utilities|Enum|Equal(Enum) _type "NewEnumerator1")) ; check if holding item and if item is default
    (if (not (Variables|Default|GetbIsOn)) ; check if the appliance is running
      (CallFunction|Fetch _Item)
      (Default|AddIngredientText (Variables|Default|GetPopupWidgetReference) _displayname))
    (elif (not (and (== _id -1) (.bIsBusy (Utilities|Struct|BreakS_Tentacle _Tentacle)))) ; Check if tentacle is busy using other appliance
      (if (Variables|Default|GetbHoldsProcessedItem) ; check if there was something that cooked
        (bind __bisable (CallFunction|CheckifAblePickUp _tentacleid))
        ;[1 1 1] getting an item out
        (if __bisable
          (bind __inventoryitem (CallFunction|Retrieve _tentacleid))
          (bind _asbp_first_person_character (Utilities|Casting|CastToBP_FirstPersonCharacter (Game|Player|GetPlayerPawn 0)))
          (Default|AddItem (Variables|/Game/Blueprints/Actor/BP_FirstPersonCharacter.BP_FirstPersonCharacter_C|GetBP_AC_Inventory _asbp_first_person_character) (.DisplayName (Utilities|Struct|BreakS_InventoryItem __inventoryitem)) _tentacleid (.ID (Utilities|Struct|BreakS_InventoryItem __inventoryitem)) (.Type (Utilities|Struct|BreakS_InventoryItem __inventoryitem)) (.DatabaseReferenceName (Utilities|Struct|BreakS_InventoryItem __inventoryitem)))
          (CallFunction|NewRecipeLearnt? (.DatabaseReferenceName (Utilities|Struct|BreakS_InventoryItem __inventoryitem)))
          (Default|SetTentacleBusy _asbp_first_person_character _tentacleid)
          (Variables|Default|SetbHoldsProcessedItem false)
          (Default|ClearIngredientText (Variables|Default|GetPopupWidgetReference))
          (Class|BPIAppliance|Off(Message) self)
          (Default|ClearIngredientText (Variables|Default|GetPopupWidgetReference))
          (else
            (if (Variables|Default|GetbIsOn) :!label _label ; check if the appliance is running
              (Variables|/Game/UI/In-game/AppliancePopup.AppliancePopup_C|SetIngredientText _popupwidgetreference "Wait bitch")
              (Utilities|FlowControl|Delay 2.0)
              (Variables|/Game/UI/In-game/AppliancePopup.AppliancePopup_C|SetIngredientText _popupwidgetreference "Cooking...")
              (elif (Utilities|Array|IsNotEmpty (Variables|Default|GetIngredientIDs)) ; If there is something in the pot
                (Class|BPIAppliance|On(Message) self)
                (Variables|/Game/UI/In-game/AppliancePopup.AppliancePopup_C|SetIngredientText (Variables|Default|GetPopupWidgetReference) "Cooking...")))))
        (else
          (goto _label))))))

(event EventFetch
  (params (_InventoryItem :type S%20Inventory%20Item%20Structure))
  (CallFunction|AddItem _InventoryItem))

(event EventBeginPlay
  (bind _asappliance_popup (Utilities|Casting|CastToAppliancePopup (UserInterface|GetWidget (Variables|Default|GetInventoryWidget)))
    (:then
      (Variables|Default|SetPopupWidgetReference _asappliance_popup))
    (:CastFailed
      (Development|PrintString "Hello"))))

(event EventOn
  (CallFunction|Turnon))

(event EventOff
  (CallFunction|TurnOff))

(fn ConstructionScript)

(fn AddItem
  (params (_Item :type S%20Inventory%20Item%20Structure))
  (bind (_id _displayname _type _holdingtentacleid) (Utilities|Struct|BreakS_InventoryItem _Item))
  (bind _returnvalue (Game|Player|GetPlayerPawn 0))
  (if (< (Utilities|Array|Length (Variables|Default|GetIngredientIDs)) (Variables|Default|GetIngredientCap))
    (Utilities|Array|Add (Variables|Default|GetIngredientIDs) _id)
    (Development|PrintString (Utilities|String|Append _displayname (Utilities|String|Append " Ingridient added to the " (Variables|Default|GetName))))
    ;[0 1 0.1702] Correct progression of interaction
    (Default|RemoveItem (Actor|GetComponentbyClass _returnvalue "/Game/Blueprints/Actor/BP_AC_Inventory.BP_AC_Inventory_C") _holdingtentacleid)
    (bind _asbp_first_person_character (Utilities|Casting|CastToBP_FirstPersonCharacter _returnvalue))
    (Default|SetTentacleFree _asbp_first_person_character _holdingtentacleid)
    (else
      (Development|PrintString "Appliance already full"))))

(fn Turnon
  (Development|PrintString "Appliance is being turned on")
  (Audio|SpawnSoundatLocation "/Game/Art/Sound/A_Stove.A_Stove" "0, 0, 0" "0, 0, 0" 1.0 1.0 0.0 0 0)
  (Variables|Default|SetbIsOn true))

(fn TurnOff
  (Development|PrintString "Appliance is being turned off")
  (Audio|SpawnSoundatLocation "/Game/Art/Sound/A_Stove.A_Stove" "0, 0, 0" "0, 0, 0" 1.0 1.0 0.0 0 0)
  (Variables|Default|SetbIsOn false))

(fn TimerFinished)

(fn CheckifAblePickUp
  (params (_TentacleID :type Integer))
  (bind __activetentacle (Class|BPIPlayerController|ActiveTentacle(Message) (Game|GetPlayerController 0)))
  (if (== __activetentacle _TentacleID)
    (bind _asbp_first_person_character (Utilities|Casting|CastToBP_FirstPersonCharacter (Game|Player|GetPlayerPawn 0)))
    (bind __bisbusy (Default|CheckTentacleBusy _asbp_first_person_character _TentacleID))
    (if __bisbusy
      (return false)
      (else
        (return true)))))

(fn NewRecipeLearnt?
  (params (text :type Name))
  (bind _returnvalue (SaveGame|LoadGamefromSlot "Slot1"))
  (bind _asmy_save_game (Utilities|Casting|CastToMySaveGame _returnvalue))
  (Variables|Default|SetSaveGameReference _asmy_save_game)
  (if (Utilities|Array|ContainsItem (Variables|/Game/MySaveGame.MySaveGame_C|GetLearntRecipeNames (Variables|Default|GetSaveGameReference)) text) ; If we haven't already learnt the recipe
    (Development|PrintString "Recipe already known")
    (else
      (Development|PrintString "Learning new recipe")
      (Utilities|Array|AddUnique (Variables|/Game/MySaveGame.MySaveGame_C|GetLearntRecipeNames (Variables|Default|GetSaveGameReference)) text)
      (bind _new_recipe_learnt_ (Default|LearnRecipe (Variables|Default|GetSaveGameReference) text))
      (SaveGame|SaveGametoSlot (Variables|Default|GetSaveGameReference) "Slot1")
      (if _new_recipe_learnt_
        (bind _returnvalue_2 (UserInterface|CreateWidget "/Game/UI/In-game/NewRecipePopup.NewRecipePopup_C"))
        (UserInterface|Viewport|AddtoViewport _returnvalue_2 0)
        (UserInterface|Animation|PlayAnimation _returnvalue_2 (Variables|/Game/UI/In-game/NewRecipePopup.NewRecipePopup_C|GetPopupAndFade _returnvalue_2) 0.0 1 "Forward" 1.0 false)))))

(fn FetchfromDatabase
  (params (_ItemName :type Name :default "None"))
  (bind _returnvalue (Utilities|GetDataTableRow "/Game/Blueprints/DT_Objects.DT_Objects" _ItemName) ; get current object we are working on
    (:then
      (return _returnvalue))))

(fn Retrieve
  (params (_ActiveTentacleID :type Integer))
  (bind _processed_item (Variables|Default|GetProcessed%20Item))
  (bind (_id _ingredientsid _name _displayname _timetocook _rewardvalue _itemtype) (Utilities|Struct|BreakS_Object _processed_item))
  (return (Utilities|Struct|MakeS_InventoryItem _id _displayname _itemtype _ActiveTentacleID _name)))

(fn RetrieveChildAttached
  (params (_Child :type BP%20A%20Ingredient%20Object%20Reference))
  (return ""))