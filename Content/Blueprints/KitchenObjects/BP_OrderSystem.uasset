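; Kitchen order manager that generates meal orders, shows them on order screens and handles serving.
; A one-second looping timer adds orders up to a cap, by time threshold or random roll, drawing a requested or random recipe from DT_Objects.
; Parallel arrays track displayed and sent orders as they fill free screens.
; SendOrder matches screen and order IDs and passes score to the game mode, which checks the level threshold once the serving limit is reached.
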(event Custom|Timer
  (params (_DeltaTime :type Float%20%28double-precision%29))
  (Utilities|FlowControl|Delay _DeltaTime)
  (CallFunction|AddOrdertoDisplayScreen))

(event EventStartOrdersComingin
  (Utilities|Time|SetTimerbyFunctionName 0 "OrderComeIn" 1.0 true)
  (bind _outactors (Actor|GetAllActorsOfClass "/Game/Blueprints/KitchenObjects/BP_AOrderScreen.BP_AOrderScreen_C"))
  (Variables|Default|SetOrderScreens _outactors)
  (bind _returnvalue (Actor|GetActorOfClass "/Game/Blueprints/KitchenObjects/Clock/BP_AClock.BP_AClock_C"))
  (Variables|Default|SetGlobalTimerRef _returnvalue))

(event EventDesiredMeal
  (params (_MealName :type Name :default "None"))
  (Variables|SetUp|SetDesiredMealName _MealName)
  (Variables|SetUp|SetbWantsDesiredMeal true))

(fn ConstructionScript
  (Variables|Ordering|SetMaxNumberOfOrders 8.0)
  (Variables|Ordering|SetChanceOfReceivingOrder 1.0)
  (Variables|Ordering|SetTimeOffsetForOrders 6e+01)
  (Variables|Ordering|SetNumberOfOrders 3.0))

(fn OrderComein
  ;[1 1 1] Printing seconds since last order
  (Variables|Ordering|SetSecondsPassedSinceLastOrder (+ (Variables|Ordering|GetSecondsPassedSinceLastOrder) 1.0))
  (if (not (>= (Variables|Ordering|GetNumberOfOrders) (Variables|Ordering|GetMaxNumberOfOrders))) ; if we didn't hit the max number of orders
    (if (>= (Variables|Ordering|GetSecondsPassedSinceLastOrder) (Variables|Ordering|GetTimeOffsetForOrders)) ; if it doesn't hit the time treshhold
      (CallFunction|FetchOrder :!label _label)
      (Variables|Ordering|SetSecondsPassedSinceLastOrder 0.0)
      (Variables|Ordering|SetNumberOfOrders (+ (Variables|Ordering|GetNumberOfOrders) 1.0))
      (elif (<= (Math|Random|RandomFloatinRange 0.0 1.0) (* (Variables|Ordering|GetChanceOfReceivingOrder) 1.15)) ; Random chance of getting the order early
        (goto _label)))))

(fn AddOrdertoDisplayScreen
  (for _array_element (Variables|Default|GetOrderScreens)
    (if (not (Variables|/Game/Blueprints/KitchenObjects/BP_AOrderScreen.BP_AOrderScreen_C|GetbHasOrder _array_element))
      (for _index (range 0 (- (Utilities|Array|Length (Variables|Default|GetOrderRecipes)) 1))
        (if (and (not (Utilities|Array|Get(acopy) (Variables|Ordering|GetOrderSent) _index)) (Math|Boolean|NORBoolean (Variables|/Game/Blueprints/KitchenObjects/BP_AOrderScreen.BP_AOrderScreen_C|GetbHasOrder _array_element) (Utilities|Array|Get(acopy) (Variables|Ordering|GetOrderProcessed) _index)))
          (Utilities|Array|SetArrayElem (Variables|Ordering|GetOrderProcessed) _index true true)
          (Default|DisplayOrder _array_element (Utilities|Array|Get(acopy) (Variables|Default|GetOrderRecipes) _index) _index)
          (Development|PrintString "===============================================================" true true "(R=1.000000,G=0.000000,B=0.932870,A=1.000000)" 3e+01))))))

(fn FetchOrder
  (if (Variables|SetUp|GetbWantsDesiredMeal)
    (bind _returnvalue (Utilities|GetDataTableRow "/Game/Blueprints/DT_Objects.DT_Objects" (Variables|SetUp|GetDesiredMealName))
      (:then
        (bind _output_get (LocalVariables|Set_TmpRecipe _returnvalue))
        (Utilities|Array|Add (Variables|Default|GetOrderRecipes) _output_get)
        (Variables|SetUp|SetbWantsDesiredMeal false)))
    (else
      (bind _outrownames (DataTable|GetDataTableRowNames "/Game/Blueprints/DT_Objects.DT_Objects"))
      (bind _returnvalue_2 (Utilities|GetDataTableRow "/Game/Blueprints/DT_Objects.DT_Objects" (Utilities|Array|Get(acopy) _outrownames (- (Utilities|Array|Get(acopy) (Variables|SetUp|GetOrderNumbers) (Math|Random|RandomIntegerinRange 0 (- (Utilities|Array|Length (Variables|SetUp|GetOrderNumbers)) 1))) 1)))
        (:then
          (bind _output_get_2 (LocalVariables|Set_TmpRecipe _returnvalue_2))
          (Utilities|Array|Add (Variables|Default|GetOrderRecipes) _output_get_2)))))
  ;[1 1 1] Additional variables for checking is order has been displayed on the scrren and if it has been already cooked and served
  (Utilities|Array|Add (Variables|Ordering|GetOrderProcessed) false)
  (Utilities|Array|Add (Variables|Ordering|GetOrderSent) false)
  (CallFunction|AddOrdertoDisplayScreen))

(fn SendOrder
  (params (_OrderID :type Integer) (_ScreenID :type Integer) (_Score :type Float%20%28double-precision%29))
  ;[1 1 1] Check is recipe matches the order and then if screen matches the serving area
  (for _array_element (Variables|Default|GetOrderScreens)
    (if (== (Variables|/Game/Blueprints/KitchenObjects/BP_AOrderScreen.BP_AOrderScreen_C|GetScreenID _array_element) _ScreenID)
      (if (== (Variables|/Game/Blueprints/KitchenObjects/BP_AOrderScreen.BP_AOrderScreen_C|GetOrderID _array_element) _OrderID)
        (Default|CleanScreen _array_element)
        (for _index (range 0 (- (Utilities|Array|Length (Variables|Ordering|GetOrderProcessed)) 1))
          ;[1 1 1] Checkif the order wasn't already sent & check if it was processed. Mark as send if true.
          (if (and (not (Utilities|Array|Get(acopy) (Variables|Ordering|GetOrderSent) _index)) (and (Utilities|Array|Get(acopy) (Variables|Ordering|GetOrderProcessed) _index) (== (Variables|/Game/Blueprints/KitchenObjects/BP_AOrderScreen.BP_AOrderScreen_C|GetOrderNumber _array_element) _index)))
            (Utilities|Array|SetArrayElem (Variables|Ordering|GetOrderSent) _index true)
            (bind _asbp_first_person_game_mode (Utilities|Casting|CastToBP_FirstPersonGameMode (Game|GetGameMode)) ; Game mode fails to cast
              (:then
                (Development|PrintString (Utilities|String|ToString(Float) _Score))
                (Default|AddScoretoHUD _asbp_first_person_game_mode _Score)
                (CallFunction|CheckifOrderLimitReached))
              (:CastFailed
                (Development|PrintString "Cast Failed -> BP_FirstPersonGameMode")))
            (else
              (Development|PrintString "Orders not processed"))))
        (else
          (Development|PrintString "Order ID's do not match")
          (CallFunction|CheckifOrderLimitReached :!label _label)))
      (else
        (Development|PrintString "Screen ID =/= ID in ServingArea")
        (goto _label)))))

(fn CheckifOrderLimitReached
  (CallFunction|Timer 3.0)
  (bind _result (Math|Float|IncrementFloat (Variables|Ordering|GetOrdersServed))
    (:%20%20
      (if (>= _result (Variables|Ordering|GetMaxOrdersServable))
        (bind _asbp_first_person_game_mode (Utilities|Casting|CastToBP_FirstPersonGameMode (Game|GetGameMode)))
        (Default|CheckScore _asbp_first_person_game_mode (Variables|Scoring|GetLevelScoreThreshold))))))