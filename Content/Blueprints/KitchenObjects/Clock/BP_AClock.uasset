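; BP_AClock is the kitchen wall clock that acts as the level timer.
; A BeginPlay Delay loop advances time one unit per second, rotates the hour and minute hands, and exposes the time through GetCurrentTime.
; At closing time it stops incoming orders in BP_OrderSystem, extends the end to an order's expiry if later, then notifies the game mode through BPI_GameMode to finish.
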(event EventLevelEnd)

(event EventBeginPlay
  (bind _returnvalue (Game|GetGameMode))
  (bind _returnvalue_2 (Actor|GetActorOfClass "/Game/Blueprints/KitchenObjects/BP_OrderSystem.BP_OrderSystem_C"))
  (Variables|Default|SetOrderSystem _returnvalue_2)
  ;[1 1 1] This here will be responsible of looking at the time - it will retrieve the time from the system
  (bind _output_get (Variables|Default|SetTimeStartRelative 5.4e+02)) ; 9:00 O'clock
  (Variables|Default|SetTimeEndRelative 5.8e+02) ; 21:00 O'clock
  (Variables|Default|SetTimeCurrentRelative _output_get)
  (Transformation|SetRelativeRotation (Variables|Default|GetSM_Hours) (Math|Rotator|MakeRotator 0.0 (* (+ (* (/ (Variables|Default|GetTimeCurrentRelative) 6e+01) 30) (/ (/ (Math|Float|Floor (* (Math|Float|%(Float) (Variables|Default|GetTimeCurrentRelative) 6e+01) 1e+02)) 100) 2.5)) -1.0) 0.0) false false :!label _label)
  (Transformation|SetRelativeRotation (Variables|Default|GetSM_Minutes) (Math|Rotator|MakeRotator 0.0 (* (/ (Math|Float|Floor (* (Math|Float|%(Float) (Variables|Default|GetTimeCurrentRelative) 6e+01) 1e+02)) 100) -6.0) 0.0) false false)
  (Utilities|FlowControl|Delay 1.0)
  (Variables|Default|SetTimeCurrentRelative (+ (Variables|Default|GetTimeCurrentRelative) 1.0))
  (if (< (Variables|Default|GetTimeCurrentRelative) (Variables|Default|GetTimeEndRelative))
    (goto _label)
    (else
      (Variables|Default|SetbAboutTofinish false)
      (if (Variables|Default|GetbAboutTofinish)
        (if (> (.OrderExpires (Utilities|Struct|BreakS_TimeOrderManagement (Utilities|Array|Get(acopy) (Variables|/Game/Blueprints/KitchenObjects/BP_OrderSystem.BP_OrderSystem_C|GetTimesForOrders (Variables|Default|GetOrderSystem)) 0))) (Variables|Default|GetTimeEndRelative)) :!label _label_2
          (Variables|Default|SetTimeEndRelative (.OrderExpires (Utilities|Struct|BreakS_TimeOrderManagement (Utilities|Array|Get(acopy) (Variables|/Game/Blueprints/KitchenObjects/BP_OrderSystem.BP_OrderSystem_C|GetTimesForOrders (Variables|Default|GetOrderSystem)) 0)))))
        (if (>= (Variables|Default|GetTimeCurrentRelative) (Variables|Default|GetTimeEndRelative))
          (if (Utilities|DoesObjectImplementInterface _returnvalue "/Game/Blueprints/Interfaces/BPI_GameMode.BPI_GameMode_C")
            (Class|BPIGameMode|FinishGame(Message) _returnvalue)
            (else
              (goto _label)))
          (else
            (goto _label)))
        (else
          (Development|PrintString "Timer end")
          (bind (_array_element _array_index) (Utilities|Array|ForEachLoopwithBreak (Variables|/Game/Blueprints/KitchenObjects/BP_OrderSystem.BP_OrderSystem_C|GetOrderProcessed (Variables|Default|GetOrderSystem)) :!label _label_3)
            (:LoopBody
              (if _array_element
                (Variables|Default|SetLast%20Order%20Index _array_index)
                (else
                  (goto _label_3 Break))))
            (:Completed
              (Class|BPIOrderSystem|StopOrdersComingin(Message) (Variables|Default|GetOrderSystem))
              (Variables|Default|SetbAboutTofinish true)
              (goto _label_2))))))))

(fn ConstructionScript)

(fn GetCurrentTime
  (return (Variables|Default|GetTimeCurrentRelative)))