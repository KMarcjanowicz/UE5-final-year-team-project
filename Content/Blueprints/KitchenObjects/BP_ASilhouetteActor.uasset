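; BP_ASilhouetteActor is a kitchen object that briefly shows a random monster silhouette with a munching animation.
; ShutterAnimation reveals one of three monster components, then plays the Munching timeline to raise and slightly enlarge the root.
; When the timeline finishes, it hides a monster by the returned ID.
; That ID comes from a separate random roll, so it can differ from the monster shown.
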(event Custom|ShutterAnimation
  (bind _returnvalue (Transformation|GetActorLocation))
  (bind (_x _y) (Math|Vector|BreakVector _returnvalue))
  (Development|PrintString "Silhuette animation" true true "(R=1.000000,G=0.000000,B=0.041855,A=1.000000)")
  (bind __randommonster (CallFunction|ChangeMonsterSilhuette))
  (bind _eating_food (Timeline|Munching PlayFromStart)
    (:Update
      (Transformation|SetRelativeTransform (Variables|Default|GetDefaultSceneRoot) (Math|Transform|MakeTransform (Math|Vector|MakeVector _x _y (Math|Float|Lerp 0.0 55.0 _eating_food)) (Transformation|GetActorRotation) (Math|Vector|MakeVector (Math|Float|Lerp 1.0 1.2 _eating_food) (Math|Float|Lerp 1.0 1.2 _eating_food) (Math|Float|Lerp 1.0 1.2 _eating_food))) false false))
    (:Finished
      (CallFunction|MakeMonsterInvisible __randommonster))))

(event EventBeginPlay)

(event Collision|EventActorBeginOverlap
  (params (OtherActor :type Actor%20Object%20Reference)))

(event EventTick
  (params (DeltaSeconds :type Float%20%28single-precision%29)))

(fn ConstructionScript)

(fn ChangeMonsterSilhuette
  (bind _returnvalue (Math|Random|RandomIntegerinRange 1 3))
  (switch int _returnvalue
    (:1
      (Rendering|SetVisibility (Variables|Default|GetMonster1) true false))
    (:2
      (Rendering|SetVisibility (Variables|Default|GetMonster2) true false))
    (:3
      (Rendering|SetVisibility (Variables|Default|GetMonster3) true false)))
  (return _returnvalue))

(fn MakeMonsterInvisible
  (params (_MonsterID :type Integer))
  (switch int _MonsterID
    (:1
      (Rendering|SetVisibility (Variables|Default|GetMonster1) false false))
    (:2
      (Rendering|SetVisibility (Variables|Default|GetMonster2) false false))
    (:3
      (Rendering|SetVisibility (Variables|Default|GetMonster3) false false))))