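; Kitchen order manager that generates recipe orders, shows them on order screens and handles serving.
; A one-second timer adds orders after a delay or by random chance, up to a cap on total orders.
; FetchOrder picks from three DT_Recipes rows, timestamps via the clock, and tracks processed/sent flags in parallel arrays for display on free screens.
; SendOrder matches screen and order IDs, clears the screen, flags orders sent, adds score and refreshes displays.
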(event EventBeginPlay
  (Utilities|Time|SetTimerbyFunctionName 0 "OrderComeIn" 1.0 true))

(event Collision|EventActorBeginOverlap
  (params (OtherActor :type Actor%20Object%20Reference)))

(event EventTick
  (params (DeltaSeconds :type Float%20%28single-precision%29)))

(fn ConstructionScript
  (Variables|Default|SetMaxNumberOfOrders 8.0)
  (Variables|Default|SetChanceOfReceivingOrder 0.2)
  (Variables|Default|SetTimeOffsetForOrders 3e+01)
  (Variables|Default|SetNumberOfOrders 0.0)
  (bind _outactors (Actor|GetAllActorsOfClass "/Game/Blueprints/Objects/KitchenObjects/BP_AOrderScreen.BP_AOrderScreen_C"))
  (Variables|Default|SetOrderScreens _outactors)
  (bind _returnvalue (Actor|GetActorOfClass "/Game/Blueprints/Objects/KitchenObjects/Clock/BP_AClock.BP_AClock_C"))
  (Variables|Default|SetGlobalTimerRef _returnvalue))

(fn OrderComein
  ;[1 1 1] Printing seconds since last order
  (Variables|Default|SetSecondsPassedSinceLastOrder (+ (Variables|Default|GetSecondsPassedSinceLastOrder) 1.0))
  (if (not (>= (Variables|Default|GetNumberOfOrders) (Variables|Default|GetMaxNumberOfOrders))) ; if we didn't hit the max number of orders
    (if (>= (Variables|Default|GetSecondsPassedSinceLastOrder) (Variables|Default|GetTimeOffsetForOrders)) ; if it doesn't hit the time treshhold
      (CallFunction|FetchOrder :!label _label) ; Random order and call to add to the order displays
      (Variables|Default|SetSecondsPassedSinceLastOrder 0.0)
      (Variables|Default|SetNumberOfOrders (+ (Variables|Default|GetNumberOfOrders) 1.0))
      (elif (<= (Math|Random|RandomFloatinRange 0.0 1.0) (* (Variables|Default|GetChanceOfReceivingOrder) 1.15)) ; Random chance of getting the order early
        (goto _label)))))

(fn AddOrdertoDisplayScreen
  (for _array_element (Variables|Default|GetOrderScreens)
    (if (not (Variables|/Game/Blueprints/Objects/KitchenObjects/BP_AOrderScreen.BP_AOrderScreen_C|GetbHasOrder _array_element))
      (for _index (range 0 (- (Utilities|Array|Length (Variables|Default|GetOrderRecipes)) 1))
        (if (Class|KismetMathLibrary|XORBoolean (Math|Boolean|NORBoolean (Variables|/Game/Blueprints/Objects/KitchenObjects/BP_AOrderScreen.BP_AOrderScreen_C|GetbHasOrder _array_element) (Utilities|Array|Get(acopy) (Variables|Default|GetOrderProcessed) _index)) (Utilities|Array|Get(acopy) (Variables|Default|GetOrderSent) _index))
          (Utilities|Array|SetArrayElem (Variables|Default|GetOrderProcessed) _index true)
          (Default|DisplayOrder _array_element (Utilities|Array|Get(acopy) (Variables|Default|GetOrderRecipes) _index)))))))

(fn FetchOrder
  (bind _output_get (LocalVariables|Set_RecipeNumber (Math|Random|RandomIntegerinRange 1 3)))
  (bind _outrownames (DataTable|GetDataTableRowNames "/Game/Blueprints/Objects/Recipes/DT_Recipes.DT_Recipes"))
  (bind _returnvalue (Utilities|GetDataTableRow "/Game/Blueprints/Objects/Recipes/DT_Recipes.DT_Recipes" (Utilities|Array|Get(acopy) _outrownames (- _output_get 1)))
    (:then
      (bind _output_get_2 (LocalVariables|Set_TmpRecipe _returnvalue))
      (bind _newparam (Default|GetCurrentTime (Variables|Default|GetGlobalTimerRef))) ; Get time when order has been placed
      (bind _structout (Utilities|Struct|SetmembersinSRecipe (Utilities|Struct|MakeSRecipe (.ID (Utilities|Struct|BreakSRecipe _output_get_2)) (.IngredientsID (Utilities|Struct|BreakSRecipe _output_get_2)) (.ToolsID (Utilities|Struct|BreakSRecipe _output_get_2)) (.Name (Utilities|Struct|BreakSRecipe _output_get_2)) (.TimeToCook (Utilities|Struct|BreakSRecipe _output_get_2)) _newparam (+ _newparam (.TimeToCook (Utilities|Struct|BreakSRecipe _output_get_2))) (.PlaceholderforStaticmeshblueprint (Utilities|Struct|BreakSRecipe _output_get_2)) (.RewardValue (Utilities|Struct|BreakSRecipe _output_get_2)))))
      (Utilities|Array|Add (Variables|Default|GetOrderRecipes) _structout)
      ;[1 1 1] Additional variables for checking is order has been displayed on the scrren and if it has been already cooked and served
      (Utilities|Array|Add (Variables|Default|GetOrderProcessed) false)
      (Utilities|Array|Add (Variables|Default|GetOrderSent) false)
      (CallFunction|AddOrdertoDisplayScreen))))

(fn SendOrder
  (params (_OrderID :type Integer) (_ScreenID :type Integer))
  ;[1 1 1] Check is recipe matches the order and then if screen matches the serving area
  (for _array_element (Variables|Default|GetOrderScreens)
    (if (== (Variables|/Game/Blueprints/Objects/KitchenObjects/BP_AOrderScreen.BP_AOrderScreen_C|GetScreenID _array_element) _ScreenID)
      (if (== (Variables|/Game/Blueprints/Objects/KitchenObjects/BP_AOrderScreen.BP_AOrderScreen_C|GetOrderID _array_element) _OrderID)
        ;[1 1 1] Checkif the order wasn't already sent & check if it was processed. Mark as send if true.
        (Default|CleanScreen _array_element)
        (for _index (range 0 (- (Utilities|Array|Length (Variables|Default|GetOrderProcessed)) 1))
          (if (and (Utilities|Array|Get(acopy) (Variables|Default|GetOrderProcessed) _index) (== (Variables|/Game/Blueprints/Objects/KitchenObjects/BP_AOrderScreen.BP_AOrderScreen_C|GetOrderID _array_element) _OrderID))
            (Utilities|Array|SetArrayElem (Variables|Default|GetOrderSent) _index true)
            (bind _asbp_first_person_game_mode (Utilities|Casting|CastToBP_FirstPersonGameMode (Game|GetGameMode))) ; Game mode fails to cast
            (Default|AddScoretoHUD _asbp_first_person_game_mode 1e+02)
            (CallFunction|AddOrdertoDisplayScreen)))))))