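; BP_AClock is a kitchen clock actor that keeps its own in-game time, starting at 9:00 on BeginPlay.
; A looping one-second Delay adds a second to the time counter and sets the pitch of the hour, minute and second hand meshes from it.
; GetCurrentTime exposes the counter in seconds; a 21:00 end time is set but not used here, and the system clock is never read.
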(event EventBeginPlay
  ;[1 1 1] This here will be responsible of looking at the time - it will retrieve the time from the system
  (bind _output_get (Variables|Default|SetTimeStartRelative 3.24e+04)) ; 9:00 O'clock
  (Variables|Default|SetTimeEndRelative 7.56e+04) ; 21:00 O'clock
  (Variables|Default|SetTimeCurrentRelative _output_get)
  (Transformation|SetRelativeRotation (Variables|Default|GetSM_HourHand) (Math|Rotator|MakeRotator 0.0 (* (+ (* (/ (Variables|Default|GetTimeCurrentRelative) 3.6e+03) 30) (/ (Math|Conversions|ToFloat(Integer) (Math|Float|Truncate (Math|Float|%(Float) (/ (Variables|Default|GetTimeCurrentRelative) 6e+01) 6e+01))) 2.0)) -1.0) 0.0) false false :!label _label)
  (Transformation|SetRelativeRotation (Variables|Default|GetSM_MinutesHand) (Math|Rotator|MakeRotator 0.0 (* (Math|Float|%(Float) (/ (Variables|Default|GetTimeCurrentRelative) 6e+01) 6e+01) -6.0) 0.0) false false)
  (Transformation|SetRelativeRotation (Variables|Default|GetSM_SecondsHand) (Math|Rotator|MakeRotator 0.0 (* (/ (Math|Float|Floor (* (Math|Float|%(Float) (Variables|Default|GetTimeCurrentRelative) 6e+01) 1e+02)) 100) -6.0) 0.0) false false)
  (Utilities|FlowControl|Delay 1.0)
  (Variables|Default|SetTimeCurrentRelative (+ (Variables|Default|GetTimeCurrentRelative) 1.0))
  (goto _label))

(fn ConstructionScript)

(fn GetCurrentTime
  (return (Variables|Default|GetTimeCurrentRelative)))