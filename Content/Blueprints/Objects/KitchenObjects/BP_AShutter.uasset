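; BP_AShutter is a kitchen shutter actor that opens and closes by snapping to preset heights.
; OpenShutter and CloseShutter set the IsOpen flag and move the actor to the open or close Z position, keeping its X and Y.
; Opening also starts a per-shutter delay event that closes it automatically after a few seconds.
; The construction script initializes each shutter as closed.
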(event Custom|CloseShutterAfterDelay
  ;[1 1 1] Custom event to have every shutter has it's own timer to close if inactive
  (if (Variables|Default|GetbIsOpen)
    (Utilities|FlowControl|Delay 5.0)
    (CallFunction|CloseShutter)))

(fn ConstructionScript
  (|CallParentFunction)
  (Variables|Default|SetbIsOpen false))

(fn OpenShutter
  (bind _self self)
  (bind _returnvalue (Transformation|GetActorTransform _self))
  (bind _location (Math|Transform|BreakTransform _returnvalue))
  (bind (_x _y) (Class|KismetMathLibrary|BreakVector3f _location))
  (if (not (Variables|Default|GetbIsOpen)) ; check if it is not open
    (Variables|Default|SetbIsOpen true)
    (Transformation|SetActorLocation (Math|Vector|MakeVector _x _y (.Z (Class|KismetMathLibrary|BreakVector3f (Variables|Default|GetOpenPos)))) false false)
    (CallFunction|CloseShutterAfterDelay)))

(fn CloseShutter
  (bind _self self)
  (bind _returnvalue (Transformation|GetActorTransform _self))
  (bind _location (Math|Transform|BreakTransform _returnvalue))
  (bind (_x _y) (Class|KismetMathLibrary|BreakVector3f _location))
  (if (Variables|Default|GetbIsOpen) ; check if it is not open
    (Variables|Default|SetbIsOpen false)
    (Transformation|SetActorLocation (Math|Vector|MakeVector _x _y (.Z (Class|KismetMathLibrary|BreakVector3f (Variables|Default|GetClosePos)))) false false)))