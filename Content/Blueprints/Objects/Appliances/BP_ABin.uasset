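; BP_ABin is a kitchen bin appliance that destroys ingredient items that touch it.
; On actor overlap it calls the parent handler, casts the other actor to BP_AInteractableItem and destroys it if its type enum marks it as an ingredient.
; Non-ingredient items and failed casts only print a debug message.
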(event EventBeginPlay
  (|CallParentFunction) ; This node is disabled and will not be called.\nDrag off pins to build functionality.
)

(event Collision|EventActorBeginOverlap
  (params (OtherActor :type Actor%20Object%20Reference))
  ;[1 1 1] Destory item (ingridient only) when colliditng with bin
  (|CallParentFunction OtherActor)
  (bind _asbp_ainteractable_item (Utilities|Casting|CastToBP_AInteractableItem OtherActor)
    (:then
      (if (Utilities|ClassIsChildOf (Utilities|GetClass OtherActor) "/Game/Blueprints/Objects/BP_AInteractableItem.BP_AInteractableItem_C")
        (if (Utilities|Enum|Equal(Enum) (Variables|/Game/Blueprints/Objects/BP_AInteractableItem.BP_AInteractableItem_C|GetType _asbp_ainteractable_item) "NewEnumerator1")
          (Actor|DestroyActor OtherActor)
          (else
            (Development|PrintString "Item is not an ingridient")))))
    (:CastFailed
      (Development|PrintString "\"Cast failed, class is not interactable object\""))))

(event EventTick
  (params (DeltaSeconds :type Float%20%28single-precision%29))
  (|CallParentFunction DeltaSeconds) ; This node is disabled and will not be called.\nDrag off pins to build functionality.
)

(fn ConstructionScript
  (|CallParentFunction))