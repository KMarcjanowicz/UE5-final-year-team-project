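; BP_AServingArea is a serving station that submits a finished dish to the order system.
; Tick polls until both CrockeryID and RecipeID are non-zero, then swaps the mesh to a placeholder material during a five-second Delay.
; It then restores the material, calls SendOrder with the recipe and station ID, and clears both IDs.
; The construction script finds and caches the BP_OrderSystem actor.
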(event EventTick
  (params (DeltaSeconds :type Float%20%28single-precision%29))
  (bind _staticmesh (Variables|Default|GetStaticMesh))
  (|CallParentFunction DeltaSeconds)
  (if (!= (Variables|Default|GetCrockeryID) 0)
    (if (!= (Variables|Default|GetRecipeID) 0)
      (Rendering|Material|SetMaterial _staticmesh 0 "/Game/StarterContent/Materials/M_Metal_Rust.M_Metal_Rust") ; Temp change material., change this to look like it's on later
      (Utilities|FlowControl|Delay 5.0) ; Playanimation for seving here
      (Rendering|Material|SetMaterial _staticmesh 0 "/Game/StarterContent/Materials/M_Wood_Walnut.M_Wood_Walnut") ; Change back to defauly material
      ;[1 1 1] Send order to order system
      (Default|SendOrder (Variables|Default|GetOrderSystem) (Variables|Default|GetRecipeID) (Variables|Default|GetID))
      (Variables|Default|SetRecipeID 0)
      (Variables|Default|SetCrockeryID 0))))

(fn ConstructionScript
  (|CallParentFunction)
  (bind _returnvalue (Actor|GetActorOfClass "/Game/Blueprints/Objects/KitchenObjects/BP_OrderSystem.BP_OrderSystem_C"))
  (Variables|Default|SetOrderSystem _returnvalue))