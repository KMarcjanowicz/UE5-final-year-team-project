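; BP_ARecipe is a recipe actor that can be picked up as an item.
; ItemPickUp runs only while the recipe is not in use: it prints the name, destroys the actor and returns its name, ID, type and database reference name.
; A SetinUse event and GetInUse function expose the in-use flag, which the construction script clears.
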(event EventBeginPlay)

(event Collision|EventActorBeginOverlap
  (params (OtherActor :type Actor%20Object%20Reference)))

(event EventTick
  (params (DeltaSeconds :type Float%20%28single-precision%29)))

(event EventSetinUse
  (params (_InUse :type Boolean))
  (Variables|Default|SetbIsInUse _InUse))

(fn ConstructionScript
  (Variables|Default|SetbIsInUse false))

(fn GetinUse
  (return (Variables|Default|GetbIsInUse)))

(fn ItemPickUp
  (if (not (Variables|Default|GetbIsInUse))
    (Development|PrintString (Variables|Default|GetName))
    (CallFunction|Destroy) ; destory actor after pick up
    (return (Variables|Default|GetName) (Variables|Default|GetID) (Variables|Default|GetType) (Variables|Default|GetDatabase%20Reference%20Name))))