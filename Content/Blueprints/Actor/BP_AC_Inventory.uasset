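; Inventory actor component that tracks which item each of the player's tentacles holds, one slot per tentacle index.
; BuildInventory fills empty placeholder slots; AddItem and RemoveItem overwrite a slot and have BP_FirstPersonGameMode update the tentacle HUD.
; RemoveItem only clears slots with a positive ID, since zero means empty and negative marks a tentacle busy with an appliance.
; GetItemActor resolves a slot's actor through the game mode's data-table lookup.
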(event EventBeginPlay)

(event EventTick
  (params (DeltaSeconds :type Float%20%28single-precision%29)))

(fn AddItem
  (params (_ItemName :type String) (_TentacleID :type Integer) (_ItemID :type Integer) (_ItemType :type E_ItemTypes%20Enum :default "NewEnumerator0") (_RefName :type Name))
  (Utilities|Array|SetArrayElem (Variables|Default|GetInventory) _TentacleID (Utilities|Struct|MakeS_InventoryItem _ItemID _ItemName _ItemType _TentacleID _RefName))
  (bind _asbp_first_person_game_mode (Utilities|Casting|CastToBP_FirstPersonGameMode (Game|GetGameMode)))
  (Default|DisplayObjectinTentacleHUD _asbp_first_person_game_mode (Utilities|Array|Get(acopy) (Variables|Default|GetInventory) _TentacleID) true))

(fn GetItem
  (params (_TentacleID :type Integer))
  (return (Utilities|Array|Get(acopy) (Variables|Default|GetInventory) _TentacleID)))

(fn RemoveItem
  (params (_TentacleID :type Integer))
  (bind _inventory (Variables|Default|GetInventory))
  (bind _output (Utilities|Array|Get(acopy) _inventory _TentacleID))
  (bind (_id _displayname _type _holdingtentacleid) (Utilities|Struct|BreakS_InventoryItem _output))
  (if (== _TentacleID _holdingtentacleid) ; check if correct tentacle
    (if (!= _id 0) ; check if not default item
      (if (> _id 0) ; check if maybe not busy by the appliance with ID -1
        (Utilities|Array|SetArrayElem (Variables|Default|GetInventory) _TentacleID (Utilities|Struct|MakeS_InventoryItem 0 "." "NewEnumerator11" _TentacleID))
        (bind _asbp_first_person_game_mode (Utilities|Casting|CastToBP_FirstPersonGameMode (Game|GetGameMode)))
        (Default|DisplayObjectinTentacleHUD _asbp_first_person_game_mode (Utilities|Array|Get(acopy) (Variables|Default|GetInventory) _TentacleID) false))
      (else
        (Development|PrintString "No item being held")))))

(fn GetItemActor
  (params (_CurrentTentacleID :type Integer))
  (bind __object (Class|BPIGameMode|RetrieveItemfromDT(Message) (Game|GetGameMode) (.DatabaseReferenceName (Utilities|Struct|BreakS_InventoryItem (Utilities|Array|Get(acopy) (Variables|Default|GetInventory) _CurrentTentacleID)))))
  (return (.BPActor (Utilities|Struct|BreakS_Object __object))))

(fn BuildInventory
  (params (_InventorySize :type Integer))
  (for _index (range 0 (- _InventorySize 1))
    (Utilities|Array|Add (Variables|Default|GetInventory) (Utilities|Struct|MakeS_InventoryItem 0 "." "NewEnumerator11" -1))))