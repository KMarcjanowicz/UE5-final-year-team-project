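; Player controller that lets the player cycle through the pawn's tentacles with the mouse wheel and opens UI widgets.
; On BeginPlay it reads the tentacle count from the pawn and shows the cursor.
; Wheel input steps the current index within bounds, without wrapping, and sends new and old indices to the GameMode.
; Key presses open a cached pause menu that pauses the game, or spawn an animated new-recipe popup.
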(event EventBeginPlay
  (Variables|Default|SetCurrentTentacle 0)
  (bind _output_get (Variables|Default|SetPlayerPawn (Game|Player|GetPlayerPawn 0)))
  (bind __numberoftentacles (Class|BPITentacles|GetNumberOfTentacles(Message) _output_get))
  (Variables|Default|SetMax%20Number%20of%20Tentacles __numberoftentacles)
  (Variables|Default|SetbShowMouseCursor true))

(event EventTick
  (params (DeltaSeconds :type Float%20%28single-precision%29)))

(event Input|MouseEvents|MouseWheelAxis
  (params (AxisValue :type Float%20%28single-precision%29))
  (bind _returnvalue (Game|GetGameMode))
  (bind _currenttentacle (Variables|Default|GetCurrentTentacle))
  (bind _output_get (Variables|Default|SetAxis%20Value AxisValue))
  (if (not (== _output_get 0.0))
    (if (> (Variables|Default|GetAxis%20Value) 0.0)
      (bind _bispossible (CallFunction|CheckTentaclesOutOfBounds -1 _currenttentacle))
      ;[1 1 1] mouse wheel down - go back on thentacle menu
      (if _bispossible
        (bind _output_get_2 (Variables|Default|SetOldTentacle (Variables|Default|GetCurrentTentacle)))
        (bind _result (Math|Integer|DecrementInt (Variables|Default|GetCurrentTentacle))
          (:%20%20
            (Class|BPIGameMode|GetActiveTentacle(Message) _returnvalue _result _output_get_2))))
      (else
        (bind _bispossible_2 (CallFunction|CheckTentaclesOutOfBounds 1 _currenttentacle))
        ;[1 1 1] if mouse whell scrolled up, it will progress on the tentacle menu
        (if _bispossible_2
          (bind _output_get_3 (Variables|Default|SetOldTentacle (Variables|Default|GetCurrentTentacle)))
          (bind _result_2 (Math|Integer|IncrementInt (Variables|Default|GetCurrentTentacle))
            (:%20%20
              (Class|BPIGameMode|GetActiveTentacle(Message) _returnvalue _result_2 _output_get_3))))))))

(event Input|KeyboardEvents|I
  (params (Key :type Key%20Structure :default "None"))
  (:Pressed
    (bind _returnvalue (UserInterface|CreateWidget "/Game/UI/In-game/NewRecipePopup.NewRecipePopup_C"))
    (UserInterface|Viewport|AddtoViewport _returnvalue 0)
    (UserInterface|Animation|PlayAnimation _returnvalue (Variables|/Game/UI/In-game/NewRecipePopup.NewRecipePopup_C|GetPopupAndFade _returnvalue) 0.0 1 "Forward" 1.0 false)))

(event Input|KeyboardEvents|0
  (params (Key :type Key%20Structure :default "None"))
  ;[1 1 1] Show pause menu
  (:Pressed
    (Utilities|IsValid (Variables|Default|GetPauseMenuReference)
      (:Is%20Valid
        _)
      (:Is%20Not%20Valid
        (bind _returnvalue (UserInterface|CreateWidget "/Game/UI/Menus/PauseMenu.PauseMenu_C"))
        (bind _output_get (Variables|Default|SetPauseMenuReference _returnvalue))))
    (UserInterface|Viewport|AddtoViewport _output_get 0)
    (Input|SetInputModeUIOnly (Game|GetPlayerController 0) _output_get "DoNotLock")
    (Game|SetGamePaused true)))

(fn ConstructionScript)

(fn CheckTentaclesOutOfBounds
  (params (_Range :type Integer) (_CurrentNo :type Integer))
  (LocalVariables|Set_CurrentTentacle _CurrentNo)
  (if (> _Range 0)
    (if (>= (LocalVariables|Get_CurrentTentacle) (- (Variables|Default|GetMax%20Number%20of%20Tentacles) 1)) ; if 1 then check if larger than max number of tentacles
      _
      (else
        (return true)))
    (elif (< (LocalVariables|Get_CurrentTentacle) 1) ; if -1 then check if is smaller than 0
      _
      (else
        (return true))))
  (return false))

(fn ActiveTentacle
  (return (Variables|Default|GetCurrentTentacle)))