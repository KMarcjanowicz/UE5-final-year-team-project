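; BP_ARat is a rat actor that spins and plays its Freebird1 audio while the cursor hovers over it.
; On BeginPlay it silences the audio, binds the cursor-over events and starts the Spinning timeline, which drives actor yaw.
; A Delay chained to the timeline's update restarts the spin from the beginning roughly every ten seconds.
; Cursor enter fades the audio in and cursor exit fades it out.
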(event Custom|Freebird
  (params (TouchedActor :type Actor%20Object%20Reference))
  (Audio|Components|Audio|FadeIn (Variables|Default|GetFreebird1) 5.0 1.0 0.0 "Linear" :!class /Script/Engine.AudioComponent))

(event Custom|Sadness
  (params (TouchedActor :type Actor%20Object%20Reference))
  (Audio|Components|Audio|FadeOut (Variables|Default|GetFreebird1) 5.0 0.0 "Linear" :!class /Script/Engine.AudioComponent))

(event EventBeginPlay
  (Audio|Components|Audio|Stop (Variables|Default|GetFreebird1))
  (EventDispatchers|BindEventtoOnEndCursorOver (delegate Custom|Sadness))
  (EventDispatchers|BindEventtoOnBeginCursorOver (delegate Custom|Freebird))
  (bind _spinning (Timeline|Spinning Play)
    (:Update
      (Transformation|SetActorRotation (Math|Rotator|MakeRotator 0.0 0.0 _spinning))
      (Utilities|FlowControl|Delay 1e+01)
      (Timeline|Spinning PlayFromStart))))

(fn ConstructionScript)