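; BP_ADispenser is a dispenser actor that hands out one configured inventory item to tentacles.
; On BeginPlay, Fetch looks up the configured item name in the DT_Objects data table, printing a message if missing, and caches the row as an inventory item struct.
; Dispense returns a copy of that cached item stamped with the requesting tentacle's ID.
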(event EventBeginPlay
  (|CallParentFunction)
  (bind __fetcheditem (CallFunction|Fetch))
  (Variables|Default|SetInventoryItemDispensed (Utilities|Struct|MakeS_InventoryItem (.ID (Utilities|Struct|BreakS_Object __fetcheditem)) (Utilities|String|ToString(Name) (.Name (Utilities|Struct|BreakS_Object __fetcheditem))) (.ItemType (Utilities|Struct|BreakS_Object __fetcheditem)) -1 (Variables|Default|GetDispencedItemDatabaseName))))

(event Collision|EventActorBeginOverlap
  (params (OtherActor :type Actor%20Object%20Reference))
  (|CallParentFunction OtherActor) ; This node is disabled and will not be called.\nDrag off pins to build functionality.
)

(event EventTick
  (params (DeltaSeconds :type Float%20%28single-precision%29))
  (|CallParentFunction DeltaSeconds) ; This node is disabled and will not be called.\nDrag off pins to build functionality.
)

(fn ConstructionScript
  (|CallParentFunction))

(fn Dispense
  (params (_TentacleID :type Integer))
  (bind _inventoryitemdispensed (Variables|Default|GetInventoryItemDispensed))
  (bind (_id _displayname _type _holdingtentacleid _databasereferencename) (Utilities|Struct|BreakS_InventoryItem _inventoryitemdispensed))
  (return (Utilities|Struct|MakeS_InventoryItem _id _displayname _type _TentacleID _databasereferencename)))

(fn Fetch
  (bind _returnvalue (Utilities|GetDataTableRow "/Game/Blueprints/DT_Objects.DT_Objects" (Variables|Default|GetDispencedItemDatabaseName))
    (:then
      (return _returnvalue))
    (:RowNotFound
      (Development|PrintString (Utilities|String|Append (Utilities|String|ToString(Name) (Variables|Default|GetDispencedItemDatabaseName)) " Not found in the Data Table")))))