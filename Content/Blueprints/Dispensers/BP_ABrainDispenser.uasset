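; BP_ABrainDispenser is a dispenser Blueprint for brain items, built on parent dispenser logic that is not shown here.
; Its construction script calls the parent, then sets the dispensed item to BP_ABrain and its database name to "Brain".
; Cursor hover events call the parent and toggle the Widget component's visibility, showing it on hover and hiding it when the cursor leaves.
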(event EventBeginPlay
  (|CallParentFunction) ; This node is disabled and will not be called.\nDrag off pins to build functionality.
)

(event Collision|EventActorBeginOverlap
  (params (OtherActor :type Actor%20Object%20Reference))
  (|CallParentFunction OtherActor) ; This node is disabled and will not be called.\nDrag off pins to build functionality.
)

(event EventTick
  (params (DeltaSeconds :type Float%20%28single-precision%29))
  (|CallParentFunction DeltaSeconds) ; This node is disabled and will not be called.\nDrag off pins to build functionality.
)

(event MouseInput|EventActorBeginCursorOver
  (|CallParentFunction)
  (Rendering|SetVisibility (Variables|Default|GetWidget) true false))

(event MouseInput|EventActorEndCursorOver
  (|CallParentFunction)
  (Rendering|SetVisibility (Variables|Default|GetWidget) false false))

(fn ConstructionScript
  (|CallParentFunction)
  (Variables|Default|SetItemDispensed "/Game/Blueprints/Ingredients/BP_ABrain.BP_ABrain_C")
  (Variables|Default|SetDispencedItemDatabaseName "Brain"))