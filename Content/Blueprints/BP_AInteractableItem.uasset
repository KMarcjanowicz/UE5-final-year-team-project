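; Interactable item actor that highlights under the cursor and can be destroyed, intended for when it is picked up.
; Cursor over and end-over events toggle the "Selected" scalar parameter on its static mesh materials.
; Separate functions, not called within this Blueprint, add or remove a duplicate outline mesh component with every slot set to an outline material.
; A Destroy event removes the actor after a short delay.
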(event Custom|Destroy
  (Utilities|FlowControl|Delay 0.1)
  (Actor|DestroyActor))

(event EventBeginPlay)

(event Collision|EventActorBeginOverlap
  (params (OtherActor :type Actor%20Object%20Reference)))

(event EventTick
  (params (DeltaSeconds :type Float%20%28single-precision%29)))

(event MouseInput|EventActorBeginCursorOver
  (Rendering|Material|SetScalarParameterValueonMaterials (Variables|Default|GetStaticMesh) "Selected" 1.0))

(event MouseInput|EventActorEndCursorOver
  (Rendering|Material|SetScalarParameterValueonMaterials (Variables|Default|GetStaticMesh) "Selected" 0.0))

(fn ConstructionScript)

(fn HighlightObjectStart
  (params (_mesh :type Static%20Mesh%20Object%20Reference))
  ;[1 1 1] Highlighting the object
  (bind _returnvalue (AddComponent|AddStaticMeshComponent false))
  (bind _output_get (Variables|Default|SetOutlineMesh _returnvalue))
  (Components|StaticMesh|SetStaticMesh _output_get _mesh)
  (for _index (range 0 (- (Utilities|Array|Length (Rendering|Material|GetMaterials (Variables|Default|GetOutlineMesh))) 1))
    (Rendering|Material|SetMaterial (Variables|Default|GetOutlineMesh) _index "/Game/LevelPrototyping/Materials/MI_Outline_Material.MI_Outline_Material")))

(fn HighlightObjectEnd
  (bind _outlinemesh (Variables|Default|GetOutlineMesh))
  (Utilities|IsValid _outlinemesh
    (:Is%20Valid
      (Components|DestroyComponent _outlinemesh))))