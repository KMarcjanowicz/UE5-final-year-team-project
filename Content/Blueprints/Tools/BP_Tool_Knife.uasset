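; Knife tool that starts its linked cutting board when the player interacts with it.
; Interact turns the board on only if the player's active tentacle is free and the board is non-empty and not already running.
; Cursor hover shows the board's inventory widget and, if the board passes its contents checks, highlights the knife through a "Selected" material parameter.
; Construction disables physics and gravity on the mesh and sets the tool type.
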(event EventBeginPlay
  (bind _asbp_first_person_character (Utilities|Casting|CastToBP_FirstPersonCharacter (Game|Player|GetPlayerPawn 0)))
  (Variables|Default|SetAs%20BP%20First%20Person%20Character _asbp_first_person_character))

(event MouseInput|EventActorBeginCursorOver
  (Rendering|SetVisibility (Variables|/Game/Blueprints/Appliances/BP_AAppliance.BP_AAppliance_C|GetInventoryWidget (Variables|CuttingBoard|GetCuttingBoard)) true false)
  (bind __bisempty (Default|CheckifEmpty (Variables|CuttingBoard|GetCuttingBoard)))
  (bind __bisholding (Default|CheckifHoldsItem (Variables|CuttingBoard|GetCuttingBoard)))
  (if (not __bisholding)
    (if (not __bisempty)
      (Rendering|Material|SetScalarParameterValueonMaterials (Variables|Default|GetStaticMesh) "Selected" 1.0))))

(event EventTick
  (params (DeltaSeconds :type Float%20%28single-precision%29)))

(event Collision|EventActorBeginOverlap
  (params (OtherActor :type Actor%20Object%20Reference)))

(event EventInteract
  (params (_TentacleID :type Integer))
  (bind _as_bp_first_person_character (Variables|Default|GetAs%20BP%20First%20Person%20Character))
  (bind __bisbusy (Default|CheckTentacleBusy _as_bp_first_person_character (Variables|/Game/Blueprints/Actor/BP_FirstPersonCharacter.BP_FirstPersonCharacter_C|GetActive%20Tentacle _as_bp_first_person_character)))
  (if (not __bisbusy)
    (bind __bisempty (Default|CheckifEmpty (Variables|CuttingBoard|GetCuttingBoard)))
    (if (not __bisempty)
      (if (not (Variables|/Game/Blueprints/Appliances/BP_AAppliance.BP_AAppliance_C|GetbIsOn (Variables|CuttingBoard|GetCuttingBoard)))
        (Default|Turnon (Variables|CuttingBoard|GetCuttingBoard))))))

(event MouseInput|EventActorEndCursorOver
  (Rendering|SetVisibility (Variables|/Game/Blueprints/Appliances/BP_AAppliance.BP_AAppliance_C|GetInventoryWidget (Variables|CuttingBoard|GetCuttingBoard)) false false)
  (Rendering|Material|SetScalarParameterValueonMaterials (Variables|Default|GetStaticMesh) "Selected" 0.0))

(fn ConstructionScript
  (|CallParentFunction)
  (Physics|SetSimulatePhysics (Variables|Default|GetStaticMesh) false)
  (Physics|SetEnableGravity (Variables|Default|GetStaticMesh) false)
  (Variables|Default|SetType "NewEnumerator13"))